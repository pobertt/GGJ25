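; Player character for the wildlife photography game, acting as an on-screen cursor that is colored per player.
; On possession it finds the floating camera, adds the input mapping and tints its cursor widget.
; Enhanced Input and gamepad stick move it on the world Y/Z plane, zeroing velocity on release.
; Left click or right trigger sphere-traces from the camera through the cursor and sends HitMessage with the player ID to the hit actor.
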(event `self.ReceivePossessed`
  (params (NewController :type "Controller Object Reference"))
  (`parent.ReceivePossessed` NewController)
  (bind _returnvalue (`GameplayStatics.GetActorOfClass` "/Game/Blueprints/BP_FloatingCamera.BP_FloatingCamera_C"))
  (set `self.Cam REF` _returnvalue)
  (bind _asbp_player_controller_wlp (cast `/Game/Blueprints/WildLifePhotography/BP_PlayerController_WLP` NewController))
  (bind _returnvalue_2 (pcsubsystem `EnhancedInputLocalPlayerSubsystem` _asbp_player_controller_wlp))
  (`/Engine/EditorBlueprintResources/StandardMacros.IsValid` _returnvalue_2
    (:`Is Valid`
      (`EnhancedInputSubsystemInterface.AddMappingContext` _returnvalue_2 "/Game/ThirdPerson/Input/IMC_Default.IMC_Default" 0 (struct))
      (`KismetSystemLibrary.PrintString` (`KismetSystemLibrary.GetDisplayName` null))
      (bind _aswb_cursor_wlp (cast `/Game/Blueprints/WildLifePhotography/WB_Cursor_WLP` (`WidgetComponent.GetWidget` (`self.Widget`))))
      (set `/Game/Blueprints/WildLifePhotography/WB_Cursor_WLP.Color` (select `/Game/Blueprints/E_Player` (`self.Player`) :`NewEnumerator0` (struct :`R` 1.0 :`A` 1.0) :`NewEnumerator1` (struct :`G` 1.0 :`A` 1.0) :`NewEnumerator2` (struct :`B` 1.0 :`A` 1.0) :`NewEnumerator3` (struct :`R` 1.0 :`G` 0.85077 :`A` 1.0) :!type "LinearColor Structure") _aswb_cursor_wlp))))

(event `Key|LeftMouseButton`
  (params (Key :type "Key Structure"))
  (bind _returnvalue (`self.K2_GetActorLocation` (`self.Cam REF`)))
  (:`Pressed`
    (bind (_outhit _returnvalue_2) (`KismetSystemLibrary.SphereTraceSingle` _returnvalue (+ (* (`KismetMathLibrary.GetForwardVector` (`KismetMathLibrary.FindLookAtRotation` _returnvalue (`SceneComponent.K2_GetComponentLocation` (`self.Widget`)))) 5000.0) _returnvalue) 10.0 "TraceTypeQuery1" :!label _label))
    (if _returnvalue_2
      (message `/Game/Blueprints/WildLifePhotography/BPI_WLP.Hit` (`.HitActor` (`GameplayStatics.BreakHitResult` _outhit)) (`self.Player`)))))

(event `Key|Gamepad_RightTrigger`
  (params (Key :type "Key Structure"))
  (:`Pressed`
    (goto _label)))

(event `EnhancedInput|/Game/ThirdPerson/Input/Actions/IA_Move`
  (params (ActionValue :type "Vector2D Structure") (ElapsedSeconds :type "Float (double-precision)") (TriggeredSeconds :type "Float (double-precision)") (InputAction :type "InputAction Object Reference" :default "/Game/ThirdPerson/Input/Actions/IA_Move.IA_Move"))
  (:`Triggered`
    (`self.AddMovementInput` (0.0 1.0 0.0) ActionValue_X)
    (`self.AddMovementInput` (0.0 0.0 1.0) ActionValue_Y))
  (:`Completed`
    (set `MovementComponent.Velocity` (0.0 0.0 0.0) (`self.CharacterMovement`))))

(event `InputVectorAxis|Gamepad_Left2D`
  (params (AxisValue :type "Vector Structure"))
  (if (and (`KismetMathLibrary.NearlyEqual_FloatFloat` AxisValue_X 0.0 0.01) (`KismetMathLibrary.NearlyEqual_FloatFloat` AxisValue_Y 0.0 0.01))
    (set `MovementComponent.Velocity` (0.0 0.0 0.0) (`self.CharacterMovement`))
    (else
      (`self.AddMovementInput` (0.0 1.0 0.0) AxisValue_X)
      (`self.AddMovementInput` (0.0 0.0 1.0) AxisValue_Y))))

(fn `UserConstructionScript`
  (`parent.UserConstructionScript`))
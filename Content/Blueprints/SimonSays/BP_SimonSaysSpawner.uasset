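; BP_SimonSaysSpawner runs the rounds of a Simon Says quick-press minigame, prompting a random key for players to match.
; Run picks a key from the Keys map, shows its texture on the WB_SimonSayser widget and unlocks every BP_SimonSaysPlayer.
; Button displays each player's press and scores it Correct or Wrong.
; A correct press or the timeout locks all players and schedules the next Run by timer.
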(event `self.ReceiveBeginPlay`
  (bind _aswb_simon_sayser (cast `/Game/Blueprints/SimonSays/WB_SimonSayser` (`WidgetComponent.GetWidget` (`self.Widget`))))
  (set `self.As WB Simon Sayser` _aswb_simon_sayser))

(event `/Game/Blueprints/SimonSays/BPI_SimonSays.Button`
  (params (Player :type "/Game/Blueprints/SimonSays/BP_SimonSaysPlayer Object Reference") (Button :type "Key Structure"))
  (if (`/Game/Blueprints/SimonSays/BP_SimonSaysPlayer.CanSelect` Player)
    (`self.ShowHitKey` Button Player)
    (if (== (`self.ActiveKey`) Button)
      (`/Game/Blueprints/SimonSays/BP_SimonSaysPlayer.Correct` Player)
      (`/Game/Blueprints/SimonSays/WB_SimonSayser.HideKey` (`self.As WB Simon Sayser`) (`/Game/Blueprints/BP_BasePlayer.Player` Player) true)
      (`KismetSystemLibrary.K2_ClearAndInvalidateTimerHandle` (`self.SimonHandle`))
      (bind _outactors (`GameplayStatics.GetAllActorsOfClass` "/Game/Blueprints/SimonSays/BP_SimonSaysPlayer.BP_SimonSaysPlayer_C"))
      (for _array_element _outactors
        (set `/Game/Blueprints/SimonSays/BP_SimonSaysPlayer.CanSelect` false _array_element)
        (`/Game/Blueprints/SimonSays/BP_SimonSaysPlayer.HideKey` _array_element))
      (`KismetSystemLibrary.K2_SetTimer` null "Run" 2.0)
      (else
        (`/Game/Blueprints/SimonSays/BP_SimonSaysPlayer.Wrong` Player)))))

(event `Run`
  (`self.SelectKey`)
  (bind _returnvalue (`KismetSystemLibrary.K2_SetTimerDelegate` (delegate `Stop`) 5.0))
  (set `self.SimonHandle` _returnvalue))

(event `Stop`
  (`/Game/Blueprints/SimonSays/WB_SimonSayser.HideKey` (`self.As WB Simon Sayser`) "NewEnumerator0" false)
  (bind _outactors (`GameplayStatics.GetAllActorsOfClass` "/Game/Blueprints/SimonSays/BP_SimonSaysPlayer.BP_SimonSaysPlayer_C"))
  (for _array_element _outactors
    (set `/Game/Blueprints/SimonSays/BP_SimonSaysPlayer.CanSelect` false _array_element)
    (`/Game/Blueprints/SimonSays/BP_SimonSaysPlayer.HideKey` _array_element))
  (`KismetSystemLibrary.K2_SetTimer` null "Run" 2.0))

(fn `SelectKey`
  (bind _keys (`self.Keys`))
  (bind _keys_2 (`BlueprintMapLibrary.Map_Keys` _keys))
  (bind _output_get (set `self.ActiveKey` (`KismetArrayLibrary.Array_Random` _keys_2)))
  (bind _values (`BlueprintMapLibrary.Map_Values` _keys))
  (bind _outactors (`GameplayStatics.GetAllActorsOfClass` "/Game/Blueprints/SimonSays/BP_SimonSaysPlayer.BP_SimonSaysPlayer_C"))
  (for _array_element _outactors
    (set `/Game/Blueprints/SimonSays/BP_SimonSaysPlayer.CanSelect` true _array_element))
  (`/Game/Blueprints/SimonSays/WB_SimonSayser.SetKey` (`self.As WB Simon Sayser`) (`|GetArrayItem` _values (`KismetArrayLibrary.Array_Find` _keys_2 _output_get))))

(fn `ShowHitKey`
  (params (Texture :type "Key Structure" :default "None") (Player :type "/Game/Blueprints/SimonSays/BP_SimonSaysPlayer Object Reference"))
  (bind _keys (`self.Keys`))
  (bind _image_41 (`/Game/Blueprints/SimonSays/WB_SimonSayserPlayer.Image_41` (`/Game/Blueprints/SimonSays/BP_SimonSaysPlayer.As WB Simon Sayser Player` Player)))
  (bind _keys_2 (`BlueprintMapLibrary.Map_Keys` _keys))
  (bind _values (`BlueprintMapLibrary.Map_Values` _keys))
  (`Widget.SetVisibility` _image_41 "Visible")
  (`Image.SetBrushFromTexture` _image_41 (`|GetArrayItem` _values (`KismetArrayLibrary.Array_Find` _keys_2 Texture)) false))

(fn `UserConstructionScript`)
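; BP_BasePlayer_HHS is a base player character for HorrorHouseScarer that handles Enhanced Input movement.
; On possession it stores a reference to the BP_FloatingCamera actor and adds the IMC_Default mapping context for a BP_PlayerController.
; IA_Move drives movement along fixed world X and Y axes and zeroes velocity on release for an instant stop.
; A leftover blackboard "Destination" write is disconnected and never runs.
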(event `self.ReceivePossessed`
  (params (NewController :type "Controller Object Reference"))
  (`parent.ReceivePossessed` NewController)
  (bind _returnvalue (`GameplayStatics.GetActorOfClass` "/Game/Blueprints/BP_FloatingCamera.BP_FloatingCamera_C"))
  (set `self.Cam REF` _returnvalue)
  (bind _asbp_player_controller (cast `/Game/Blueprints/BP_PlayerController` NewController))
  (bind _returnvalue_2 (pcsubsystem `EnhancedInputLocalPlayerSubsystem` _asbp_player_controller))
  (`/Engine/EditorBlueprintResources/StandardMacros.IsValid` _returnvalue_2
    (:`Is Valid`
      (`EnhancedInputSubsystemInterface.AddMappingContext` _returnvalue_2 "/Game/ThirdPerson/Input/IMC_Default.IMC_Default" 0 (struct)))))

(event `EnhancedInput|/Game/ThirdPerson/Input/Actions/IA_Move`
  (params (ActionValue :type "Vector2D Structure") (ElapsedSeconds :type "Float (double-precision)") (TriggeredSeconds :type "Float (double-precision)") (InputAction :type "InputAction Object Reference" :default "/Game/ThirdPerson/Input/Actions/IA_Move.IA_Move"))
  (:`Triggered`
    (`self.AddMovementInput` (0.0 1.0 0.0) ActionValue_X)
    (`self.AddMovementInput` (1.0 0.0 0.0) ActionValue_Y))
  (:`Completed`
    (set `MovementComponent.Velocity` (0.0 0.0 0.0) (`self.CharacterMovement`))))

(fn `UserConstructionScript`
  (`parent.UserConstructionScript`))
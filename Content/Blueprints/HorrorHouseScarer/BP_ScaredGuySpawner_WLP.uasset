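; A spawner actor for the horror house scarer game that periodically produces scared guy AI pawns.
; On BeginPlay it starts a looping timer, with an interval picked randomly once, that spawns BP_Scaredguy_HHS running BT_ScaredGuy_HHS at its start component.
; Each spawned pawn receives the spawner's end component as the Destination object in its blackboard.
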(event `self.ReceiveBeginPlay`
  (`KismetSystemLibrary.K2_SetTimerDelegate` (delegate `ScaredGuySpawn`) (`KismetMathLibrary.RandomFloatInRange` 3.0 6.0) true))

(event `ScaredGuySpawn`
  (bind _returnvalue (`AIBlueprintHelperLibrary.SpawnAIFromClass` "/Game/Blueprints/HorrorHouseScarer/BP_Scaredguy_HHS.BP_Scaredguy_HHS_C" "/Game/Blueprints/HorrorHouseScarer/BT_ScaredGuy_HHS.BT_ScaredGuy_HHS" (`SceneComponent.K2_GetComponentLocation` (`self.BP_StartComponent_WLP`)) (struct) false null))
  (`BlackboardComponent.SetValueAsObject` (`AIBlueprintHelperLibrary.GetBlackboard` (`Pawn.GetController` _returnvalue)) "Destination" (`self.BP_EndComponent_WLP`)))

(fn `UserConstructionScript`)
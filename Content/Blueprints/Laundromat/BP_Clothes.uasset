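; BP_Clothes is a laundry item in the Laundromat game, attached by position to its owner, BP_LaundromatLarry.
; One tick after BeginPlay it picks a random garment mesh and one of three clothing types, shown as black, grey or white material.
; The type is meant to decide which machine it belongs in.
; Every tick it teleports to the world location of Larry's Widget component.
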(event `self.ReceiveBeginPlay`
  (bind _cube (`self.Cube`))
  (`KismetSystemLibrary.DelayUntilNextTick`)
  (bind _asbp_laundromat_larry (cast `/Game/Blueprints/Laundromat/BP_LaundromatLarry` (`self.GetOwner`)))
  (set `self.As BP Laundromat Larry` _asbp_laundromat_larry)
  (`StaticMeshComponent.SetStaticMesh` (`self.Cube`) (select `int` (`KismetMathLibrary.RandomIntegerInRange` 0 4) :`0` "/Game/Assets/Laundromat/Static_Meshes/SM_Gloves.SM_Gloves" :`1` "/Game/Assets/Laundromat/Static_Meshes/SM_Hat.SM_Hat" :`2` "/Game/Assets/Laundromat/Static_Meshes/SM_Socks.SM_Socks" :`3` "/Game/Assets/Laundromat/Static_Meshes/SM_Sweater.SM_Sweater" :`4` "/Game/Assets/Laundromat/Static_Meshes/SM_Trousers.SM_Trousers" :!type "StaticMesh Object Reference"))
  (`self.K2_SetActorLocation` (`SceneComponent.K2_GetComponentLocation` (`/Game/Blueprints/Laundromat/BP_LaundromatLarry.Widget` _asbp_laundromat_larry)) false true)
  (set `self.Exists?` true)
  (bind _output_get (set `self.ClothingType` (`KismetMathLibrary.RandomIntegerInRange` 0 2)))
  (switch `int` _output_get
    (:`0`
      ;[1 1 1] Sets material and by extension which machine it should go into
      (`PrimitiveComponent.SetMaterial` _cube 0 "/Game/Blueprints/Laundromat/M_Black.M_Black"))
    (:`1`
      (`PrimitiveComponent.SetMaterial` _cube 0 "/Game/Blueprints/Laundromat/M_Grey.M_Grey"))
    (:`2`
      (`PrimitiveComponent.SetMaterial` _cube 0 "/Game/Blueprints/Laundromat/M_White.M_White"))))

(event `self.ReceiveTick`
  (params (DeltaSeconds :type "Float (single-precision)"))
  (bind _as_bp_laundromat_larry (`self.As BP Laundromat Larry`))
  (`/Engine/EditorBlueprintResources/StandardMacros.IsValid` _as_bp_laundromat_larry
    (:`Is Valid`
      (`self.K2_SetActorLocation` (`SceneComponent.K2_GetComponentLocation` (`/Game/Blueprints/Laundromat/BP_LaundromatLarry.Widget` _as_bp_laundromat_larry)) false true))))

(fn `UserConstructionScript`)
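; BP_WashingMachine is a laundromat washing machine that scores how players sort clothes by type.
; When clicked with a valid clothes item, it compares the item's ClothingType to its own Type, adds or subtracts a point for that player, then destroys the item.
; The construction script sets the cube's material from Type, so each of the three machine types looks different.
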(event `/Game/Blueprints/Laundromat/BPI_Laundromat.Clicked`
  (params (Player :type "/Game/Blueprints/E_Player Enum" :default "NewEnumerator0") (Clothes :type "/Game/Blueprints/Laundromat/BP_Clothes Object Reference"))
  (`/Engine/EditorBlueprintResources/StandardMacros.IsValid` Clothes
    (:`Is Valid`
      (if (== (`/Game/Blueprints/Laundromat/BP_Clothes.ClothingType` Clothes) (`self.Type`))
        (`/Game/Blueprints/FL_Functions.Add Score` Player 1)
        (else
          (`/Game/Blueprints/FL_Functions.Add Score` Player -1)))
      (`self.K2_DestroyActor` Clothes))))

(fn `UserConstructionScript`
  (bind _cube (`self.Cube`))
  (switch `int` (`self.Type`)
    (:`0`
      (`PrimitiveComponent.SetMaterial` _cube 0 "/Game/LevelPrototyping/Materials/M_PrototypeGrid.M_PrototypeGrid"))
    (:`1`
      (`PrimitiveComponent.SetMaterial` _cube 0 "/Game/LevelPrototyping/Materials/M_Solid.M_Solid"))
    (:`2`
      (`PrimitiveComponent.SetMaterial` _cube 0 "/Game/LevelPrototyping/Materials/MI_Solid_Blue.MI_Solid_Blue"))))
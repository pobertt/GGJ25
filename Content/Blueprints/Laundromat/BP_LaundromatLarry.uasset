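; BP_LaundromatLarry is a possessable player in a laundromat game who steers a cursor to handle laundry from a basket.
; On possession it caches its child-actor basket and floating camera, using a throwaway WBP_Cursor to assign its widget component's owning local player.
; The left stick slides that widget.
; Right trigger sphere-traces from the camera through it, sending Clicked with player and clothing to its basket or a washing machine.
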(event `self.ReceivePossessed`
  (params (NewController :type "Controller Object Reference"))
  (`parent.ReceivePossessed` NewController)
  (`PrimitiveComponent.SetCastShadow` (`self.Widget`) false)
  (bind _asbp_basket (cast `/Game/Blueprints/Laundromat/BP_Basket` (`ChildActorComponent.ChildActor` (`self.ChildActor`))))
  (bind _output_get (set `self.As BP Basket` _asbp_basket))
  (`self.SetOwner` _output_get self)
  (bind _returnvalue (`GameplayStatics.GetActorOfClass` "/Game/Blueprints/BP_FloatingCamera.BP_FloatingCamera_C"))
  (set `self.Camref` _returnvalue)
  (`KismetSystemLibrary.DelayUntilNextTick`)
  (`UserWidget.SetOwningPlayer` (`WidgetComponent.GetWidget` (`self.Widget`)) (`self.As BP Player Controller`))
  (bind _returnvalue_2 (`|CreateWidget` "/Game/Blueprints/PopUpBandits/WBP_Cursor.WBP_Cursor_C" (`GameplayStatics.GetPlayerController` (select `/Game/Blueprints/E_Player` (`self.Player`) :`NewEnumerator1` 1 :`NewEnumerator2` 2 :`NewEnumerator3` 3))))
  (`WidgetComponent.SetOwnerPlayer` (`self.Widget`) (`Widget.GetOwningLocalPlayer` _returnvalue_2))
  (`Widget.RemoveFromParent` _returnvalue_2))

(event `Key|Gamepad_RightTrigger`
  (params (Key :type "Key Structure"))
  (bind _as_bp_basket (`self.As BP Basket`))
  (bind _returnvalue (`SceneComponent.K2_GetComponentLocation` (`/Game/Blueprints/BP_FloatingCamera.Camera` (`self.Camref`))))
  (:`Pressed`
    (bind _outhit (`KismetSystemLibrary.SphereTraceSingle` _returnvalue (+ _returnvalue (* (`KismetMathLibrary.GetDirectionUnitVector` _returnvalue (`SceneComponent.K2_GetComponentLocation` (`self.Widget`))) 1000.0)) 3.0 "TraceTypeQuery1"))
    (bind (_bblockinghit _binitialoverlap _time _distance _location _impactpoint _normal _impactnormal _physmat _hitactor) (`GameplayStatics.BreakHitResult` _outhit))
    (if (or (== _hitactor _as_bp_basket) (== (`GameplayStatics.GetObjectClass` _hitactor) "/Game/Blueprints/Laundromat/BP_WashingMachine.BP_WashingMachine_C"))
      (message `/Game/Blueprints/Laundromat/BPI_Laundromat.Clicked` _hitactor (`self.Player`) (`/Game/Blueprints/Laundromat/BP_Basket.Clothing Item` _as_bp_basket)))))

(event `InputVectorAxis|Gamepad_Left2D`
  (params (AxisValue :type "Vector Structure"))
  (`SceneComponent.K2_AddRelativeLocation` (`self.Widget`) (`KismetMathLibrary.MakeVector` 0.0 (* AxisValue_X 3.0) (* AxisValue_Y 3.0)) false false))

(fn `UserConstructionScript`
  (`parent.UserConstructionScript`))
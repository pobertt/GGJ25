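; Pizza-making station in the pizza shop where the player builds a pizza on spawned dough and submits it against the customer order.
; Interact activates the hit component, using OnComponentActivated as a button to add ingredients or submit.
; Submitting attaches ingredients overlapping a temporary sphere to the dough and checks their tags appear in the game mode's order.
; The result triggers a finished message or wrong-order widget, then a timeline moves the dough away before respawn.
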(event `self.ReceiveBeginPlay`
  (bind _outactors (`GameplayStatics.GetAllActorsOfClass` "/Game/Blueprints/BP_BasePlayer.BP_BasePlayer_C"))
  (bind _asbp_base_player (cast `/Game/Blueprints/BP_BasePlayer` (`.ReturnValue` (`GameplayStatics.FindNearestActor` (`self.K2_GetActorLocation`) _outactors))))
  (set `self.As BP Base Player` _asbp_base_player)
  (bind _asbp_pizza_shop_gm (cast `/Game/Blueprints/PizzaShop/BP_PizzaShopGM` (`GameplayStatics.GetGameMode`)))
  (set `self.As BP Pizza Shop GM` _asbp_pizza_shop_gm)
  (`SceneComponent.K2_SetRelativeRotation` (`self.pepperoni_pot`) (`KismetMathLibrary.MakeRotator` 0.0 0.0 (`KismetMathLibrary.RandomFloatInRange` -5.0 5.0)) false false)
  (`SceneComponent.K2_SetRelativeRotation` (`self.cheese_pot`) (`KismetMathLibrary.MakeRotator` 0.0 0.0 (`KismetMathLibrary.RandomFloatInRange` -5.0 5.0)) false false)
  (`SceneComponent.K2_SetRelativeRotation` (`self.mushroom_pot`) (`KismetMathLibrary.MakeRotator` 0.0 0.0 (`KismetMathLibrary.RandomFloatInRange` -5.0 5.0)) false false)
  (`SceneComponent.K2_SetRelativeRotation` (`self.tomatosauce_pot`) (`KismetMathLibrary.MakeRotator` 0.0 0.0 (`KismetMathLibrary.RandomFloatInRange` -5.0 5.0)) false false)
  (`self.SpawnDough`))

(event `/Game/Blueprints/PizzaShop/BPI_PizzaShop.Interact`
  (params (Hit :type "PrimitiveComponent Object Reference"))
  (if (`self.CanMake`)
    (`ActorComponent.Activate` Hit false)))

(event `self.TomatoSauce.OnComponentActivated`
  (params (Component :type "ActorComponent Object Reference") (bReset :type Boolean))
  (`AddComponent|NODE_AddBP_PizzaIngredient-0` :`DesiredMesh` "/Game/Assets/Pizza_Shop/Static_Meshes/tomato_base.tomato_base" :`Name` "Sauce")
  (`ActorComponent.Deactivate` Component))

(event `self.Mushroom.OnComponentActivated`
  (params (Component :type "ActorComponent Object Reference") (bReset :type Boolean))
  (`AddComponent|NODE_AddBP_PizzaIngredient-1` :`DesiredMesh` "/Game/Assets/Pizza_Shop/Static_Meshes/mushroom.mushroom" :`Name` "Mushroom")
  (`ActorComponent.Deactivate` Component))

(event `self.Cheese.OnComponentActivated`
  (params (Component :type "ActorComponent Object Reference") (bReset :type Boolean))
  (`AddComponent|NODE_AddBP_PizzaIngredient-2` :`DesiredMesh` "/Game/Assets/Pizza_Shop/Static_Meshes/cheese.cheese" :`Name` "Cheese")
  (`ActorComponent.Deactivate` Component))

(event `self.Pepperoni.OnComponentActivated`
  (params (Component :type "ActorComponent Object Reference") (bReset :type Boolean))
  (`AddComponent|NODE_AddBP_PizzaIngredient-3` :`DesiredMesh` "/Game/Assets/Pizza_Shop/Static_Meshes/pepperoni.pepperoni" :`Name` "Pepperoni")
  (`ActorComponent.Deactivate` Component))

(event `self.Pizza.OnComponentActivated`
  (params (Component :type "ActorComponent Object Reference") (bReset :type Boolean))
  (`self.Check`)
  (bind _correct_ (`self.CompareOrder`))
  (set `self.CanMake` false)
  (if _correct_
    (message `/Game/Blueprints/PizzaShop/BPI_PizzaShop.Finished` (`GameplayStatics.GetGameMode`) (`/Game/Blueprints/BP_BasePlayer.Player` (`self.As BP Base Player`)))
    (`ActorComponent.Deactivate` Component)
    (`self.Restart` true)
    (else
      (bind _returnvalue (`|CreateWidget` "/Game/Blueprints/PizzaShop/WB_WrongOrder.WB_WrongOrder_C" (`/Game/Blueprints/BP_BasePlayer.As BP Player Controller` (`self.As BP Base Player`))))
      (`UserWidget.AddToPlayerScreen` _returnvalue 0)
      (`ActorComponent.Deactivate` Component)
      (`self.Restart` false))))

(event `Restart`
  (params (`Success?` :type Boolean))
  (bind _dough (`self.Dough`))
  (bind _meshes (`self.Meshes`))
  (`PrimitiveComponent.SetSimulatePhysics` (`self.Dough`) false)
  (if `Success?`
    (bind (_direction _tl) (`Timeline|Timeline` :!via `PlayFromStart` :!label _label)
      (:`Update`
        (if `Success?`
          (`SceneComponent.K2_AddLocalOffset` _dough (`KismetMathLibrary.MakeVector` 0.0 0.0 _tl) false false)
          (else
            (`SceneComponent.K2_AddLocalOffset` _dough (`KismetMathLibrary.MakeVector` 0.0 _tl) false false))))
      (:`Finished`
        (for _array_element _meshes
          (`ActorComponent.K2_DestroyComponent` _array_element))
        (`KismetArrayLibrary.Array_Clear` _meshes)
        (`ActorComponent.K2_DestroyComponent` (`self.Dough`))
        (`KismetSystemLibrary.K2_SetTimer` null "SpawnDough" (`KismetMathLibrary.SelectFloat` 1.5 0.5 `Success?`))))
    (else
      (goto _label :!via `ReverseFromEnd`))))

(fn `Check`
  (bind _returnvalue (`AddComponent|NODE_AddSphereComponent-1`))
  (`SceneComponent.K2_AttachToComponent` _returnvalue (`self.Dough`) "None" "SnapToTarget" "SnapToTarget" "SnapToTarget" true)
  (for _array_element (`self.Meshes`)
    (if (`PrimitiveComponent.IsOverlappingComponent` _returnvalue _array_element)
      (`PrimitiveComponent.SetSimulatePhysics` _array_element false)
      (`SceneComponent.K2_AttachToComponent` _array_element (`self.Dough`) "None" "KeepWorld" "KeepWorld" "KeepWorld" true)
      (bind _output (`|GetArrayItem` (`ActorComponent.ComponentTags` _array_element)))
      (`KismetArrayLibrary.Array_Add` (`self.UsedIngredients`) _output)
      (`KismetSystemLibrary.PrintString` (`KismetStringLibrary.Conv_NameToString` _output))))
  (`ActorComponent.K2_DestroyComponent` _returnvalue))

(fn `CompareOrder`
  (returns (`Correct?` :type Boolean))
  (for (_array_element _array_index) (`self.UsedIngredients`)
    (if (`KismetArrayLibrary.Array_Contains` (`/Game/Blueprints/PizzaShop/BP_PizzaShopGM.CustomerOrder` (`self.As BP Pizza Shop GM`)) _array_element)
      (`KismetArrayLibrary.Array_Remove` (`self.UsedIngredients`) _array_index)
      (else
        (`KismetArrayLibrary.Array_Clear` (`self.UsedIngredients`))
        (return false))))
  (`KismetArrayLibrary.Array_Clear` (`self.UsedIngredients`))
  (return true))

(fn `SpawnDough`
  (bind _returnvalue (`AddComponent|NODE_AddStaticMeshComponent-1` :`RelativeTransform` (`SceneComponent.GetRelativeTransform` (`self.SpawnPoint`))))
  (`StaticMeshComponent.SetStaticMesh` _returnvalue "/Game/Assets/Pizza_Shop/Static_Meshes/pizzacrust.pizzacrust")
  (`PrimitiveComponent.SetSimulatePhysics` _returnvalue true)
  (set `self.Dough` _returnvalue)
  (set `self.CanMake` true))

(fn `UserConstructionScript`)
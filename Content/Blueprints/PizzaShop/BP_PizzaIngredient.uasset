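; BP_PizzaIngredient represents one ingredient on a BP_PizzaTable, which it expects as its owner, and spawns that ingredient's physical mesh.
; On BeginPlay it adds a static mesh component to the table at the SpawnPoint transform, randomly jittering location, rotation and scale.
; The mesh gets the desired model, damped physics and ignores Visibility traces, then is tagged with the ingredient's Name and appended to the table's Meshes array.
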(event `self.ReceiveBeginPlay`
  (bind _asbp_pizza_table (cast `/Game/Blueprints/PizzaShop/BP_PizzaTable` (`self.GetOwner`)))
  (bind _output_get (set `self.As BP Pizza Table` _asbp_pizza_table))
  (bind _spawnpoint (`/Game/Blueprints/PizzaShop/BP_PizzaTable.SpawnPoint` _output_get))
  (bind (_relativerotation_roll _relativerotation_pitch _relativerotation_yaw) (`KismetMathLibrary.BreakRotator` (`SceneComponent.RelativeRotation` _spawnpoint)))
  (bind _returnvalue (`|AddComponentByClass` _output_get "/Script/Engine.StaticMeshComponent" false (`KismetMathLibrary.MakeTransform` (+ (`SceneComponent.RelativeLocation` _spawnpoint) (`KismetMathLibrary.RandomFloatInRange` -5.0 5.0)) (`KismetMathLibrary.MakeRotator` (+ _relativerotation_roll (`KismetMathLibrary.RandomFloatInRange` -25.0 25.0)) (+ _relativerotation_pitch (`KismetMathLibrary.RandomFloatInRange` -25.0 25.0)) (+ _relativerotation_yaw (`KismetMathLibrary.RandomFloatInRange` -25.0 25.0))) (+ (`SceneComponent.RelativeScale3D` _spawnpoint) (`KismetMathLibrary.RandomFloatInRange` -0.1 0.1)))))
  (set `self.Mesh` _returnvalue)
  (`StaticMeshComponent.SetStaticMesh` (`self.Mesh`) (`self.DesiredMesh`))
  (`PrimitiveComponent.SetCollisionObjectType` (`self.Mesh`) "ECC_WorldStatic")
  (`PrimitiveComponent.SetAngularDamping` (`self.Mesh`) 5.0)
  (`PrimitiveComponent.SetLinearDamping` (`self.Mesh`) 2.5)
  (`PrimitiveComponent.SetSimulatePhysics` (`self.Mesh`) true)
  (`PrimitiveComponent.SetCollisionResponseToChannel` (`self.Mesh`) "ECC_Visibility" "ECR_Ignore")
  (`KismetArrayLibrary.Array_Add` (`ActorComponent.ComponentTags` (`self.Mesh`)) (`self.Name`))
  (`KismetArrayLibrary.Array_Add` (`/Game/Blueprints/PizzaShop/BP_PizzaTable.Meshes` (`self.As BP Pizza Table`)) (`self.Mesh`)))
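; Game mode for the pizza shop minigame, where players fill randomly generated customer orders to score.
; At extra start it rolls a random ingredient list and shows the order widget.
; When a player finishes, it awards a point and removes the order for that player in the widget.
; Timed events then restart every pizza table not belonging to that player and, a second later, roll and display a new order.
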(event `self.ReceiveBeginPlay`
  (`parent.ReceiveBeginPlay`))

(event `/Game/Blueprints/PizzaShop/BPI_PizzaShop.Finished`
  (params (Player :type "/Game/Blueprints/E_Player Enum" :default "NewEnumerator0"))
  (`/Game/Blueprints/FL_Functions.Add Score` Player 1)
  (`/Game/Blueprints/PizzaShop/WB_Order.RemoveOrder` (`self.Widget`) Player)
  (`KismetSystemLibrary.K2_SetTimerDelegate` (delegate `RestartPlayers`) 1.0))

(event `RestartPlayers`
  (bind _outactors (`GameplayStatics.GetAllActorsOfClass` "/Game/Blueprints/PizzaShop/BP_PizzaTable.BP_PizzaTable_C"))
  (for _array_element _outactors
    (if (not (`|EnumEquality` (`/Game/Blueprints/BP_BasePlayer.Player` (`/Game/Blueprints/PizzaShop/BP_PizzaTable.As BP Base Player` _array_element)) (stale `/Game/Blueprints/PizzaShop/BPI_PizzaShop.Finished` Player)))
      (`/Game/Blueprints/PizzaShop/BP_PizzaTable.Restart` _array_element false)))
  (`KismetSystemLibrary.K2_SetTimerDelegate` (delegate `NewOrder`) 1.0))

(event `self.ExtraStart`
  (`self.RandomOrder`)
  (bind _returnvalue (`|CreateWidget` "/Game/Blueprints/PizzaShop/WB_Order.WB_Order_C"))
  (bind _output_get (set `self.Widget` _returnvalue))
  (`UserWidget.AddToViewport` _output_get 0))

(event `NewOrder`
  (`self.RandomOrder`)
  (`/Game/Blueprints/PizzaShop/WB_Order.NewOrder` (`self.Widget`)))

(fn `RandomOrder`
  (`KismetArrayLibrary.Array_Clear` (`self.CustomerOrder`))
  (for _ (range (+ (`KismetMathLibrary.RandomIntegerInRange` 1 4) 1))
    (`KismetArrayLibrary.Array_Add` (`self.CustomerOrder`) (`KismetArrayLibrary.Array_Random` (`self.AllIngredientTypes`)))))

(fn `UserConstructionScript`
  (`parent.UserConstructionScript`))
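; Player pawn for a pit crew minigame, where each of up to four players turns bolts on their own car.
; On possession it colors the cursor widget per player, assigns its owning player through a temporary widget, and spawns a car that slides into place.
; The left stick moves the cursor; changing right-stick input rotates it and sphere-traces from the camera through it to turn the bolt hit.
; Done awards that player a point.
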(event `self.ReceivePossessed`
  (params (NewController :type "Controller Object Reference"))
  (`parent.ReceivePossessed` NewController)
  (bind _aswb_pit_crew_cursor (cast `/Game/Blueprints/PitCrew/WB_PitCrewCursor` (`WidgetComponent.GetWidget` (`self.Widget`))))
  (bind _output_get (set `self.As WB Pit Crew Cursor` _aswb_pit_crew_cursor))
  (set `/Game/Blueprints/PitCrew/WB_PitCrewCursor.Color` (select `/Game/Blueprints/E_Player` (`self.Player`) :`NewEnumerator0` (struct :`R` 1.0 :`G` 0.018721 :`A` 1.0) :`NewEnumerator1` (struct :`R` 0.126081 :`G` 1.0 :`A` 1.0) :`NewEnumerator2` (struct :`B` 1.0 :`A` 1.0) :`NewEnumerator3` (struct :`R` 1.0 :`G` 0.883365 :`A` 1.0) :!type "LinearColor Structure") _output_get)
  (bind _returnvalue (`|CreateWidget` "/Game/Blueprints/PitCrew/WB_PitCrewCursor.WB_PitCrewCursor_C" (`GameplayStatics.GetPlayerController` (select `/Game/Blueprints/E_Player` (`self.Player`) :`NewEnumerator1` 1 :`NewEnumerator2` 2 :`NewEnumerator3` 3))))
  (`WidgetComponent.SetOwnerPlayer` (`self.Widget`) (`Widget.GetOwningLocalPlayer` _returnvalue))
  (`Widget.RemoveFromParent` _returnvalue)
  (bind _returnvalue_2 (`|SpawnActorFromClass` "/Game/Blueprints/PitCrew/BP_PitCrewCar.BP_PitCrewCar_C" (`SceneComponent.K2_GetComponentToWorld` (`self.CarSpawn`)) "AlwaysSpawn" "MultiplyWithRoot" null null))
  (bind _output_get_2 (set `self.CarREF` _returnvalue_2))
  (`self.SetOwner` _output_get_2 self)
  (bind (_direction _newtrack_0) (`Timeline|Timeline` :!via `PlayFromStart`)
    (:`Update`
      (`self.K2_SetActorLocation` _returnvalue_2 (`KismetMathLibrary.VLerp` (`SceneComponent.K2_GetComponentLocation` (`self.CarSpawn`)) (`SceneComponent.K2_GetComponentLocation` (`self.CarStop`)) _newtrack_0) false false))))

(event `InputVectorAxis|Gamepad_Left2D`
  (params (AxisValue :type "Vector Structure"))
  (`SceneComponent.K2_AddWorldOffset` (`self.Widget`) (`KismetMathLibrary.MakeVector` 0.0 (/ AxisValue_X 2.0) (/ AxisValue_Y 2.0)) false false))

(event `InputVectorAxis|Gamepad_Right2D`
  (params (AxisValue :type "Vector Structure"))
  (bind _returnvalue (`SceneComponent.K2_GetComponentLocation` (`self.Camera`)))
  (if (not (`KismetMathLibrary.Vector_IsNearlyZero` AxisValue 0.6))
    (if (not (== AxisValue (`self.Axis`) :`ErrorTolerance` 0.05))
      (`/Game/Blueprints/PitCrew/WB_PitCrewCursor.Rotate` (`self.As WB Pit Crew Cursor`))
      (bind (_outhit _returnvalue_2) (`KismetSystemLibrary.SphereTraceSingle` _returnvalue (+ _returnvalue (* (`KismetMathLibrary.GetDirectionUnitVector` _returnvalue (`SceneComponent.K2_GetComponentLocation` (`self.Widget`))) 500.0)) 3.0 "TraceTypeQuery2"))
      (if _returnvalue_2
        (`/Game/Blueprints/PitCrew/BP_PitCrewCar.RotateBolt` (`self.CarREF`) (`.HitComponent` (`GameplayStatics.BreakHitResult` _outhit)))
        (set `self.Axis` AxisValue :!label _label))
      (else
        (goto _label)))
    (else
      (goto _label))))

(event `/Game/Blueprints/PitCrew/BPI_PitCrew.Done`
  (`/Game/Blueprints/FL_Functions.Add Score` (`self.Player`) 1))

(fn `UserConstructionScript`
  (`parent.UserConstructionScript`))
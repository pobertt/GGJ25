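; Checkpoint actor for the ambulance minigame that halts the player's ambulance when it enters the Box trigger.
; On overlap it detaches the ambulance's spring arm, disables its input, waits briefly, then checks its score against a threshold.
; The score branch leads nowhere, the widget creation nodes are disconnected, and UpdateScore is empty, so no result is shown.
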(event `self.Box.OnComponentBeginOverlap`
  (params (OverlappedComponent :type "PrimitiveComponent Object Reference") (OtherActor :type "Actor Object Reference") (OtherComp :type "PrimitiveComponent Object Reference") (OtherBodyIndex :type Integer) (bFromSweep :type Boolean) (SweepResult :type "HitResult Structure (by ref)"))
  (bind _asbp_taxi (cast `/Game/Blueprints/AmbulanceMiniGame/BP_Ambulance` OtherActor))
  (`SceneComponent.K2_DetachFromComponent` (`/Game/Blueprints/AmbulanceMiniGame/BP_Ambulance.SpringArm` _asbp_taxi) "KeepRelative" "KeepRelative" "KeepRelative" true)
  (`self.DisableInput` _asbp_taxi null)
  (`KismetSystemLibrary.Delay` 1.0)
  (if (> (`/Game/Blueprints/AmbulanceMiniGame/BP_Ambulance.Score` _asbp_taxi) 4999)
    _))

(fn `UserConstructionScript`)
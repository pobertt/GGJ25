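; Player-controlled ambulance for the ambulance minigame, built around drifting for score.
; Enhanced Input gas applies impulses to the car body, snapping its rotation straight when not drifting.
; While gas is held, left/right drift inputs add side impulses, interpolate the body's rotation, spawn smoke at two spheres and play a sound, occasionally with a random extra.
; Tick adds score while drifting; releasing gas or calling stopscore ends the drift state.
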(event `self.ReceiveBeginPlay`
  (bind _asplayer_controller (cast `PlayerController` (`self.GetController`)))
  (bind _returnvalue (pcsubsystem `EnhancedInputLocalPlayerSubsystem` _asplayer_controller))
  (`/Engine/EditorBlueprintResources/StandardMacros.IsValid` _returnvalue
    (:`Is Valid`
      (`EnhancedInputSubsystemInterface.AddMappingContext` _returnvalue "/Game/Blueprints/AmbulanceMiniGame/IMC_Ambulance.IMC_Ambulance" 0 (struct))
      (set `self.is drifting` false))))

(event `EnhancedInput|/Game/Blueprints/AmbulanceMiniGame/IA_GAS`
  (params (ActionValue :type "Vector2D Structure") (ElapsedSeconds :type "Float (double-precision)") (TriggeredSeconds :type "Float (double-precision)") (InputAction :type "InputAction Object Reference" :default "/Game/Blueprints/AmbulanceMiniGame/IA_GAS.IA_GAS"))
  (bind _gas_impulse (`self.Gas Impulse`))
  (bind _carbodyy (`self.CarBodyy`))
  (:`Triggered`
    (set `self.IsMovingForward?` true)
    (`PrimitiveComponent.AddImpulse` _carbodyy _gas_impulse "None" false)
    (`PrimitiveComponent.AddAngularImpulseInDegrees` _carbodyy _gas_impulse "None" false)
    (if (not (`self.is drifting`))
      (`SceneComponent.K2_SetRelativeRotation` :`self` (`self.CarBodyy`))
      (`/Engine/EditorBlueprintResources/StandardMacros.DoOnce` false
        (:`Completed`
          (`GameplayStatics.PlaySound2D` null 1.0 1.0 0.0 null null)
          (`/Engine/EditorBlueprintResources/StandardMacros.DoOnce` false
            (:`Completed`
              (`GameplayStatics.PlaySound2D` null 1.0 1.0 0.0 null null)))))))
  (:`Completed`
    (set `self.IsMovingForward?` false)
    (set `self.is drifting` false)))

(event `EnhancedInput|/Game/Blueprints/AmbulanceMiniGame/IA_DRIFTL`
  (params (ActionValue :type "Vector2D Structure") (ElapsedSeconds :type "Float (double-precision)") (TriggeredSeconds :type "Float (double-precision)") (InputAction :type "InputAction Object Reference" :default "/Game/Blueprints/AmbulanceMiniGame/IA_DRIFTL.IA_DRIFTL"))
  (bind _drift_impulse_l (`self.Drift Impulse L`))
  (bind _carbodyy (`self.CarBodyy`))
  (:`Triggered`
    (if (`self.IsMovingForward?`)
      (set `self.is drifting` true)
      (`PrimitiveComponent.AddImpulse` _carbodyy _drift_impulse_l "None" true)
      (`PrimitiveComponent.AddAngularImpulseInDegrees` _carbodyy _drift_impulse_l "None" false)
      (`SceneComponent.K2_SetRelativeRotation` (`self.CarBodyy`) (`KismetMathLibrary.RInterpTo` (`SceneComponent.RelativeRotation` (`self.CarBodyy`)) (struct :`Yaw` -75.0) (`GameplayStatics.GetWorldDeltaSeconds`) 3.0) false false)
      (`KismetSystemLibrary.PrintString` "nice drift")
      (`|ExecutionSequence`
        (:`then_0`
          (`|ExecutionSequence`
            (:`then_0`
              (`|SpawnActorFromClass` "/Game/Blueprints/AmbulanceMiniGame/BP_smoke.BP_smoke_C" (`KismetMathLibrary.Conv_VectorToTransform` (`SceneComponent.K2_GetComponentLocation` (`self.Sphere2`))) "Undefined" "MultiplyWithRoot" null null))
            (:`then_1`
              (`|SpawnActorFromClass` "/Game/Blueprints/AmbulanceMiniGame/BP_smoke.BP_smoke_C" (`KismetMathLibrary.Conv_VectorToTransform` (`SceneComponent.K2_GetComponentLocation` (`self.Sphere3`))) "Undefined" "MultiplyWithRoot" null null))))
        (:`then_1`
          (`/Engine/EditorBlueprintResources/StandardMacros.DoOnce` false :!label _label
            (:`Completed`
              (`GameplayStatics.PlaySound2D` null 1.0 1.0 0.0 null null)
              (if (select `int` (`KismetMathLibrary.RandomIntegerInRange` 0 7) :`0` false :`1` false :`2` false :`3` false :`4` false :`5` false :`6` false :`7` true)
                (`GameplayStatics.PlaySound2D` null 1.0 1.0 0.0 null null))))))))
  (:`Completed`
    (goto _label :!via `Reset`)))

(event `EnhancedInput|/Game/Blueprints/AmbulanceMiniGame/IA_DRIFTR`
  (params (ActionValue :type "Vector2D Structure") (ElapsedSeconds :type "Float (double-precision)") (TriggeredSeconds :type "Float (double-precision)") (InputAction :type "InputAction Object Reference" :default "/Game/Blueprints/AmbulanceMiniGame/IA_DRIFTR.IA_DRIFTR"))
  (bind _drift_impulse_r (`self.Drift Impulse R`))
  (bind _carbodyy (`self.CarBodyy`))
  (:`Triggered`
    (if (`self.IsMovingForward?`)
      (set `self.is drifting` true)
      (`PrimitiveComponent.AddImpulse` _carbodyy _drift_impulse_r "None" true)
      (`PrimitiveComponent.AddAngularImpulseInDegrees` _carbodyy _drift_impulse_r "None" false)
      (`SceneComponent.K2_SetRelativeRotation` (`self.CarBodyy`) (`KismetMathLibrary.RInterpTo` (`SceneComponent.RelativeRotation` (`self.CarBodyy`)) (struct :`Yaw` 75.0) (`GameplayStatics.GetWorldDeltaSeconds`) 3.0) false false)
      (`KismetSystemLibrary.PrintString` "nice drift")
      (`|ExecutionSequence`
        (:`then_0`
          (`|ExecutionSequence`
            (:`then_0`
              (`|SpawnActorFromClass` "/Game/Blueprints/AmbulanceMiniGame/BP_smoke.BP_smoke_C" (`KismetMathLibrary.Conv_VectorToTransform` (`SceneComponent.K2_GetComponentLocation` (`self.Sphere2`))) "Undefined" "MultiplyWithRoot" null null))
            (:`then_1`
              (`|SpawnActorFromClass` "/Game/Blueprints/AmbulanceMiniGame/BP_smoke.BP_smoke_C" (`KismetMathLibrary.Conv_VectorToTransform` (`SceneComponent.K2_GetComponentLocation` (`self.Sphere3`))) "Undefined" "MultiplyWithRoot" null null))))
        (:`then_1`
          (`/Engine/EditorBlueprintResources/StandardMacros.DoOnce` false :!label _label_2
            (:`Completed`
              (`GameplayStatics.PlaySound2D` null 1.0 1.0 0.0 null null)
              (if (select `int` (`KismetMathLibrary.RandomIntegerInRange` 0 7) :`0` false :`1` false :`2` false :`3` false :`4` false :`5` false :`6` false :`7` true)
                (`GameplayStatics.PlaySound2D` null 1.0 1.0 0.0 null null))))))))
  (:`Completed`
    (goto _label_2 :!via `Reset`)))

(event `self.ReceiveTick`
  (params (DeltaSeconds :type "Float (single-precision)"))
  (if (`self.is drifting`)
    (set `self.Score` (+ (`self.Score`) 10))))

(event `stop score`
  (set `self.is drifting` false))

(fn `UserConstructionScript`)
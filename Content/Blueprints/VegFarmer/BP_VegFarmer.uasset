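; Player-controlled farmer pawn for a carrot-pulling minigame, which works through the carrots tagged for its player.
; On possession it claims those carrots and targets the nearest; right-stick movement and alternating trigger presses send yank messages to it.
; Done adds a point, launches the carrot with physics, then slides the farmer along Y to retarget the nearest remaining one.
; When none remain, it disables input and shows the player-finished widget.
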(event `self.ReceivePossessed`
  (params (NewController :type "Controller Object Reference"))
  (`parent.ReceivePossessed` NewController)
  (bind _outactors (`GameplayStatics.GetAllActorsOfClassWithTag` "/Game/Blueprints/VegFarmer/BP_Carrot.BP_Carrot_C" (select `/Game/Blueprints/E_Player` (`self.Player`) :`NewEnumerator0` "Player1" :`NewEnumerator1` "Player2" :`NewEnumerator2` "Player3" :`NewEnumerator3` "Player4" :!type "Name")))
  (bind _output_get (set `self.Carrots` _outactors))
  (for _array_element _output_get
    (`self.SetOwner` _array_element self))
  (bind _asbp_carrot (cast `/Game/Blueprints/VegFarmer/BP_Carrot` (`.ReturnValue` (`GameplayStatics.FindNearestActor` (`self.K2_GetActorLocation`) (`self.Carrots`)))))
  (set `self.CurrentCarrot` _asbp_carrot))

(event `InputVectorAxis|Gamepad_Right2D`
  (params (AxisValue :type "Vector Structure"))
  (if (not (`KismetMathLibrary.Vector_IsNearlyZero` AxisValue 0.5))
    (if (not (== AxisValue (`self.Axis`) :`ErrorTolerance` 0.5))
      (message `/Game/Blueprints/VegFarmer/BPI_VegFarmer.Yanking` (`self.CurrentCarrot`))))
  (set `self.Axis` AxisValue))

(event `Key|Gamepad_LeftTrigger`
  (params (Key :type "Key Structure"))
  (:`Pressed`
    (if (not (== Key (`self.Key`)))
      (set `self.Key` Key)
      (message `/Game/Blueprints/VegFarmer/BPI_VegFarmer.Yanking` (`self.CurrentCarrot`)))))

(event `Key|Gamepad_RightTrigger`
  (params (Key :type "Key Structure"))
  (:`Pressed`
    (if (not (== Key (`self.Key`)))
      (set `self.Key` Key)
      (message `/Game/Blueprints/VegFarmer/BPI_VegFarmer.Yanking` (`self.CurrentCarrot`)))))

(event `/Game/Blueprints/VegFarmer/BPI_VegFarmer.Done`
  (bind _returnvalue (`self.K2_GetActorLocation`))
  (bind _carrots (`self.Carrots`))
  (bind _carrot (`/Game/Blueprints/VegFarmer/BP_Carrot.Carrot` (`self.CurrentCarrot`)))
  (`/Game/Blueprints/FL_Functions.Add Score` (`self.Player`) 1)
  (`PrimitiveComponent.SetSimulatePhysics` _carrot true)
  (`PrimitiveComponent.AddImpulse` _carrot (750.0 0.0 3000.0) "None" false)
  (`KismetArrayLibrary.Array_Remove` _carrots (`KismetArrayLibrary.Array_Find` _carrots (`self.CurrentCarrot`)))
  (set `self.CurrentCarrot` null)
  (set `self.NextLoc` (+ _returnvalue (0.0 135.0 0.0)))
  (set `self.CurrLoc` _returnvalue)
  (if (`KismetArrayLibrary.Array_IsEmpty` (`self.Carrots`))
    (`self.DisableInput` (`self.As BP Player Controller`))
    (bind _returnvalue_2 (`|CreateWidget` "/Game/Blueprints/WB_PlayerFinished.WB_PlayerFinished_C" null (`self.Player`)))
    (`UserWidget.AddToViewport` _returnvalue_2 0)
    (else
      (bind (_direction _newtrack_0) (`Timeline|Timeline` :!via `PlayFromStart`)
        (:`Update`
          (`self.K2_SetActorLocation` (`KismetMathLibrary.VLerp` (`self.CurrLoc`) (`self.NextLoc`) _newtrack_0)))
        (:`Finished`
          (bind _asbp_carrot (cast `/Game/Blueprints/VegFarmer/BP_Carrot` (`.ReturnValue` (`GameplayStatics.FindNearestActor` (`self.K2_GetActorLocation`) (`self.Carrots`)))))
          (set `self.CurrentCarrot` _asbp_carrot))))))

(fn `UserConstructionScript`
  (`parent.UserConstructionScript`))
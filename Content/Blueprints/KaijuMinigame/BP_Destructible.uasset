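; BP_Destructible is a breakable prop for the Kaiju minigame that reacts when a player kaiju runs into it.
; The first kaiju overlap with its Box starts a three-second lifespan, sends BreakMessage to the kaiju if it implements BPI_collision, then destroys the Box.
; When FractureCube reports a Chaos break, it starts ignoring the Destructible collision channel.
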(event `self.Box.OnComponentBeginOverlap`
  (params (OverlappedComponent :type "PrimitiveComponent Object Reference") (OtherActor :type "Actor Object Reference") (OtherComp :type "PrimitiveComponent Object Reference") (OtherBodyIndex :type Integer) (bFromSweep :type Boolean) (SweepResult :type "HitResult Structure (by ref)"))
  (bind _asbp_base_player_kaiju (cast `/Game/Blueprints/KaijuMinigame/BP_BasePlayerKaiju` OtherActor))
  (`/Engine/EditorBlueprintResources/StandardMacros.DoOnce` false
    (:`Completed`
      (`self.SetLifeSpan` 3.0)
      (if (`KismetSystemLibrary.DoesImplementInterface` _asbp_base_player_kaiju "/Game/Blueprints/KaijuMinigame/BPI_collision.BPI_collision_C")
        (`KismetSystemLibrary.PrintString` "breakinng")
        (message `/Game/Blueprints/KaijuMinigame/BPI_collision.Break` _asbp_base_player_kaiju)
        (`ActorComponent.K2_DestroyComponent` (`self.Box`))))))

(event `self.FractureCube.OnChaosBreakEvent`
  (params (BreakEvent :type "ChaosBreakEvent Structure (by ref)"))
  (`PrimitiveComponent.SetCollisionResponseToChannel` (`self.FractureCube`) "ECC_Destructible" "ECR_Ignore"))

(fn `UserConstructionScript`)
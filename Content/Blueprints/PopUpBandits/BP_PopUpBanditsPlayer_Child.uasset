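; Player pawn for the Pop-Up Bandits shooting game, controlling a colored aiming cursor for one of four players.
; The left stick slides the widget component in world space.
; Right trigger or left click sphere-traces from the shared floating camera through the cursor, sending the hit actor a HitMessage with the player ID.
; On possession, it colors the cursor, finds the camera and assigns widget ownership through a temporary cursor widget.
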(event `Key|Gamepad_RightTrigger`
  (params (Key :type "Key Structure"))
  (bind _returnvalue (`SceneComponent.K2_GetComponentLocation` (`/Game/Blueprints/BP_FloatingCamera.Camera` (`self.Camref`))))
  (:`Pressed`
    (bind (_outhit _returnvalue_2) (`KismetSystemLibrary.SphereTraceSingle` _returnvalue (+ _returnvalue (* (`KismetMathLibrary.GetDirectionUnitVector` _returnvalue (`SceneComponent.K2_GetComponentLocation` (`self.Widget`))) 3000.0)) 3.0 "TraceTypeQuery1" :!label _label))
    (if _returnvalue_2
      (message `/Game/Blueprints/PopUpBandits/BPI_PopUpB.Hit` (`.HitActor` (`GameplayStatics.BreakHitResult` _outhit)) (`self.Player`)))))

(event `Key|LeftMouseButton`
  (params (Key :type "Key Structure"))
  (:`Pressed`
    (goto _label)))

(event `self.ReceivePossessed`
  (params (NewController :type "Controller Object Reference"))
  (`parent.ReceivePossessed` NewController)
  (`KismetSystemLibrary.DelayUntilNextTick`)
  (bind _aswbp_cursor (cast `/Game/Blueprints/PopUpBandits/WBP_Cursor` (`WidgetComponent.GetWidget` (`self.Widget`))))
  (bind _output_get (set `self.As Cursor` _aswbp_cursor))
  (set `/Game/Blueprints/PopUpBandits/WBP_Cursor.Color` (select `/Game/Blueprints/E_Player` (`self.Player`) :`NewEnumerator0` (struct :`R` 1.0 :`G` 0.018721 :`A` 1.0) :`NewEnumerator1` (struct :`R` 0.126081 :`G` 1.0 :`A` 1.0) :`NewEnumerator2` (struct :`B` 1.0 :`A` 1.0) :`NewEnumerator3` (struct :`R` 1.0 :`G` 0.883365 :`A` 1.0) :!type "LinearColor Structure") _output_get)
  (bind _returnvalue (`|CreateWidget` "/Game/Blueprints/PopUpBandits/WBP_Cursor.WBP_Cursor_C" (`GameplayStatics.GetPlayerController` (select `/Game/Blueprints/E_Player` (`self.Player`) :`NewEnumerator1` 1 :`NewEnumerator2` 2 :`NewEnumerator3` 3))))
  (`WidgetComponent.SetOwnerPlayer` (`self.Widget`) (`Widget.GetOwningLocalPlayer` _returnvalue))
  (`Widget.RemoveFromParent` _returnvalue)
  (bind _returnvalue_2 (`GameplayStatics.GetActorOfClass` "/Game/Blueprints/BP_FloatingCamera.BP_FloatingCamera_C"))
  (set `self.Camref` _returnvalue_2))

(event `InputVectorAxis|Gamepad_Left2D`
  (params (AxisValue :type "Vector Structure"))
  (`SceneComponent.K2_AddWorldOffset` (`self.Widget`) (`KismetMathLibrary.MakeVector` (* (/ AxisValue_X 1.0) -1.0) 0.0 (/ AxisValue_Y 1.0)) false false))

(fn `UserConstructionScript`
  (`parent.UserConstructionScript`))
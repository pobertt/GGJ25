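; Child game mode for the PopUpBandits game that resets pop-ups and displays the Bandits value.
; The Reset event passes through a Do Once gate, then re-randomizes and resets each pop-up in the array it receives.
; ResetReset re-arms that gate so another reset can run.
; Tick prints Bandits every frame under a fixed key.
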(event `self.ReceiveTick`
  (params (DeltaSeconds :type "Float (single-precision)"))
  (`KismetSystemLibrary.PrintString` (`KismetStringLibrary.Conv_IntToString` (`self.Bandits`)) true true (struct :`G` 0.66 :`B` 1.0 :`A` 1.0) 2.0 "1"))

(event `/Game/Blueprints/PopUpBandits/BPI_PopUpB.Reset`
  (params (PopUp :type "Array of /Game/Blueprints/PopUpBandits/BP_PopUp Object Reference (by ref)"))
  (`/Engine/EditorBlueprintResources/StandardMacros.DoOnce` false :!label _label
    (:`Completed`
      (for _array_element PopUp
        (`/Game/Blueprints/PopUpBandits/BP_PopUp.SetRandomPopUp` _array_element)
        (`/Game/Blueprints/PopUpBandits/BP_PopUp.ResetAll` _array_element)))))

(event `ResetReset`
  (goto _label :!via `Reset`))

(fn `UserConstructionScript`
  (`parent.UserConstructionScript`))
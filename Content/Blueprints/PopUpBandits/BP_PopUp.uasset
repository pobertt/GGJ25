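; BP_PopUp is a shootable pop-up target in the Pop-Up Bandits minigame, randomly a red Bandit or a green Civilian via a dynamic material color.
; Hitting a Bandit adds score, hitting a Civilian subtracts it, and either flips the cube away with a rotation Timeline.
; The game mode counts live Bandits; when none remain, every pop-up resets with new random roles, rerolling if it finds zero Bandits.
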(event `self.ReceiveBeginPlay`
  (`self.Rotate`)
  (bind _asbp_pop_up_bandits_game_mode_child (cast `/Game/Blueprints/PopUpBandits/BP_PopUpBanditsGameMode_Child` (`GameplayStatics.GetGameMode`)))
  (set `self.GamemodeRef` _asbp_pop_up_bandits_game_mode_child)
  (bind _returnvalue (`GameplayStatics.GetActorOfClass` "/Game/Blueprints/PopUpBandits/BP_PopUpBanditsPlayer_Child.BP_PopUpBanditsPlayer_Child_C"))
  (set `self.PlayerRef` _returnvalue)
  (bind _returnvalue_2 (`KismetMaterialLibrary.CreateDynamicMaterialInstance` "/Game/Blueprints/PopUpBandits/M_BanditColor_Inst.M_BanditColor_Inst"))
  (bind _output_get (set `self.Mat` _returnvalue_2))
  (`PrimitiveComponent.SetMaterial` (`self.Cube`) 0 _output_get)
  (bind _outactors (`GameplayStatics.GetAllActorsOfClass` "BP_PopUp_C"))
  (set `self.PopUpArray` _outactors))

(event `SetRandomPopUp`
  (bind _mat (`self.Mat`))
  (bind _output_get (set `self.E_PopUp` (select `bool` (`KismetMathLibrary.RandomBoolWithWeight` 0.33) :`false` "NewEnumerator0" :`true` "NewEnumerator1" :!type "/Game/Blueprints/PopUpBandits/E_PopUp Enum")))
  (switch `/Game/Blueprints/PopUpBandits/E_PopUp` _output_get
    (:`NewEnumerator0`
      (`MaterialInstanceDynamic.SetVectorParameterValue` _mat "BaseColor" (struct :`R` 1.0 :`G` 0.024081 :`A` 1.0))
      (`/Engine/EditorBlueprintResources/StandardMacros.IncrementInt` (`/Game/Blueprints/PopUpBandits/BP_PopUpBanditsGameMode_Child.Bandits` (`self.GamemodeRef`))))
    (:`NewEnumerator1`
      (`MaterialInstanceDynamic.SetVectorParameterValue` _mat "BaseColor" (struct :`R` 0.063561 :`G` 1.0 :`A` 1.0)))))

(event `/Game/Blueprints/PopUpBandits/BPI_PopUpB.Hit`
  (params (Player :type "/Game/Blueprints/E_Player Enum" :default "NewEnumerator0"))
  (if (not (`self.Hit?`))
    (switch `/Game/Blueprints/PopUpBandits/E_PopUp` (`self.E_PopUp`)
      (:`NewEnumerator0`
        (`/Game/Blueprints/FL_Functions.Add Score` Player 1)
        (`/Engine/EditorBlueprintResources/StandardMacros.DecrementInt` (`/Game/Blueprints/PopUpBandits/BP_PopUpBanditsGameMode_Child.Bandits` (`self.GamemodeRef`))
          (:`  `
            (set `self.Hit?` true)
            (`self.HitArray`)
            (`self.Rotate`))))
      (:`NewEnumerator1`
        (`/Game/Blueprints/FL_Functions.Add Score` Player -1)
        (set `self.Hit?` true)
        (`self.HitArray`)
        (`self.Rotate`)))))

(event `Rotate`
  (bind (_direction _fyvalue) (`Timeline|Timeline` :!label _label)
    (:`Update`
      (`SceneComponent.K2_SetRelativeRotation` (`self.Cube`) (`KismetMathLibrary.MakeRotator` _fyvalue 0.0 -90.0) false false))))

(event `ResetAll`
  (`|ExecutionSequence`
    (:`then_0`
      (goto _label))
    (:`then_1`
      (`KismetSystemLibrary.Delay` 0.25)
      (`self.SetRandomPopUp`)
      (`self.ResetIfAllCiv`)
      (set `self.Hit?` false)
      (goto _label :!via `Reverse`))))

(event `ResetIfAllCiv`
  (`KismetSystemLibrary.DelayUntilNextTick`)
  (if (<= (`/Game/Blueprints/PopUpBandits/BP_PopUpBanditsGameMode_Child.Bandits` (`self.GamemodeRef`)) 0)
    (`self.ResetAll`)))

(fn `HitArray`
  (locals (ArrayIndex :type Integer :default 0) (E_Type :type "Array of /Game/Blueprints/PopUpBandits/E_PopUp Enum"))
  (if (<= (`/Game/Blueprints/PopUpBandits/BP_PopUpBanditsGameMode_Child.Bandits` (`self.GamemodeRef`)) 0)
    (for _array_element (`self.PopUpArray`)
      (`self.ResetAll` _array_element))))

(fn `UserConstructionScript`)
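; Player pawn for the PopUpBandits game that lets the player hit pop-up targets with the mouse.
; A left click deprojects the cursor from player controller 0, runs a Visibility line trace with persistent debug drawing, and calls HitPopUp on any BP_PopUp struck.
; An example event forwards a score to AddScore.
; Possession prints the controller's name, and the BP_PopUp lookup on BeginPlay goes unused.
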(event `self.ReceiveBeginPlay`
  (`GameplayStatics.GetActorOfClass` "/Game/Blueprints/PopUpBandits/BP_PopUp.BP_PopUp_C"))

(event `self.ReceivePossessed`
  (params (NewController :type "Controller Object Reference"))
  (`KismetSystemLibrary.PrintString` (`KismetSystemLibrary.GetDisplayName` NewController)))

(event `ExampleAddScore`
  (params (Score :type Integer))
  (`/Game/Blueprints/FL_Functions.Add Score` (`self.Player`) Score))

(event `Key|LeftMouseButton`
  (params (Key :type "Key Structure"))
  (bind (_worldlocation _worlddirection) (`PlayerController.DeprojectMousePositionToWorld` (`GameplayStatics.GetPlayerController` 0)))
  (:`Pressed`
    (bind _outhit (`KismetSystemLibrary.LineTraceSingle` :`Start` _worldlocation :`End` (+ _worldlocation (* _worlddirection 10000.0)) :`TraceChannel` "TraceTypeQuery1" :`DrawDebugType` "Persistent"))
    (bind _asbp_pop_up (cast `/Game/Blueprints/PopUpBandits/BP_PopUp` (`.HitActor` (`GameplayStatics.BreakHitResult` _outhit))))
    (`/Game/Blueprints/PopUpBandits/BP_PopUp.HitPopUp` _asbp_pop_up)))

(fn `UserConstructionScript`)
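; Udder actor that visualizes milking, with separately triggered right and left sides.
; MilkUddersRight and MilkUddersLeft each use a FlipFlop to toggle milking on their side with every call.
; Toggling on activates that side's milk effect and plays a timeline that drives the Z scale of its sphere.
; Toggling off deactivates the effect and reverses the timeline to undo the scaling.
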(event `MilkUddersRight`
  (bind _ns_milk1 (`self.NS_Milk1`))
  (bind _sphere1 (`self.Sphere1`))
  (bind (_relativescale3d_x _relativescale3d_y) (`KismetMathLibrary.BreakVector` (`SceneComponent.RelativeScale3D` _sphere1)))
  (`/Engine/EditorBlueprintResources/StandardMacros.FlipFlop`
    (:`A`
      (`ActorComponent.Activate` _ns_milk1 false)
      (bind (_direction _newtrack_0) (`Timeline|Timeline` :!label _label)
        (:`Update`
          (`SceneComponent.SetRelativeScale3D` _sphere1 (`KismetMathLibrary.MakeVector` _relativescale3d_x _relativescale3d_y _newtrack_0)))))
    (:`B`
      (`ActorComponent.Deactivate` _ns_milk1)
      (goto _label :!via `Reverse`))))

(event `MilkUddersLeft`
  (bind _sphere2 (`self.Sphere2`))
  (bind _ns_milk (`self.NS_Milk`))
  (bind (_relativescale3d_x _relativescale3d_y) (`KismetMathLibrary.BreakVector` (`SceneComponent.RelativeScale3D` _sphere2)))
  (`/Engine/EditorBlueprintResources/StandardMacros.FlipFlop`
    (:`A`
      (`ActorComponent.Activate` _ns_milk false)
      (bind (_direction _newtrack_0) (`Timeline|Timeline_0` :!label _label_2)
        (:`Update`
          (`SceneComponent.SetRelativeScale3D` _sphere2 (`KismetMathLibrary.MakeVector` _relativescale3d_x _relativescale3d_y _newtrack_0)))))
    (:`B`
      (`ActorComponent.Deactivate` _ns_milk)
      (goto _label_2 :!via `Reverse`))))

(fn `UserConstructionScript`)
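; Player character for an udder-milking race minigame, where players mash the gamepad triggers to fill a bucket.
; On possession it binds to the nearest udders and bucket and caches the game mode.
; Each left or right trigger press milks that side, increments the bucket's fill and nudges it upward.
; A full bucket locks input, awards score by finishing place and registers the player with the game mode.
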(event `Key|Gamepad_RightTrigger`
  (params (Key :type "Key Structure"))
  (bind _bucket (`self.Bucket`))
  (bind _player (`self.Player`))
  (bind (_returnvalue_x _returnvalue_y _returnvalue_z) (`KismetMathLibrary.BreakVector` (`self.K2_GetActorLocation` _bucket)))
  (bind _fill (`/Game/Blueprints/MilkUdders/BP_Bucket.Fill` (`self.Bucket`)))
  (bind _players (`/Game/Blueprints/MilkUdders/BP_MilkUddersGamemode.Players` (`self.As BP Milk Udders Gamemode`)))
  (:`Pressed`
    (if (not (`self.Done?`))
      (`/Game/Blueprints/MilkUdders/BP_Udders.MilkUddersRight` (`self.Udders`))
      (set `/Game/Blueprints/MilkUdders/BP_Bucket.Fill` (+ _fill 1) (`self.Bucket`))
      (`self.K2_SetActorLocation` _bucket (`KismetMathLibrary.MakeVector` _returnvalue_x _returnvalue_y (+ _returnvalue_z 0.25)) false false)
      (if (>= _fill 100.0)
        (set `self.Done?` true :!label _label)
        (`/Game/Blueprints/FL_Functions.Add Score` _player (select `int` (`KismetArrayLibrary.Array_Length` _players) :`0` 15 :`1` 10 :`2` 5 :`3` 0))
        (`KismetArrayLibrary.Array_Add` _players _player)))))

(event `Key|Gamepad_LeftTrigger`
  (params (Key :type "Key Structure"))
  (bind _bucket (`self.Bucket`))
  (bind _bucket_2 (`self.Bucket`))
  (bind (_returnvalue_x _returnvalue_y _returnvalue_z) (`KismetMathLibrary.BreakVector` (`self.K2_GetActorLocation` _bucket)))
  (:`Pressed`
    (if (not (`self.Done?`))
      (`/Game/Blueprints/MilkUdders/BP_Udders.MilkUddersLeft` (`self.Udders`))
      (set `/Game/Blueprints/MilkUdders/BP_Bucket.Fill` (+ (`/Game/Blueprints/MilkUdders/BP_Bucket.Fill` _bucket_2) 1) _bucket_2)
      (`self.K2_SetActorLocation` _bucket (`KismetMathLibrary.MakeVector` _returnvalue_x _returnvalue_y (+ _returnvalue_z 0.25)) false false)
      (if (>= (`/Game/Blueprints/MilkUdders/BP_Bucket.Fill` (`self.Bucket`)) 100.0)
        (goto _label)))))

(event `self.ReceivePossessed`
  (params (NewController :type "Controller Object Reference"))
  (`parent.ReceivePossessed` NewController)
  (bind _asbp_milk_udders_gamemode (cast `/Game/Blueprints/MilkUdders/BP_MilkUddersGamemode` (`GameplayStatics.GetGameMode`)))
  (set `self.As BP Milk Udders Gamemode` _asbp_milk_udders_gamemode)
  (bind _outactors (`GameplayStatics.GetAllActorsOfClass` "/Game/Blueprints/MilkUdders/BP_Udders.BP_Udders_C"))
  (bind _asbp_udders (cast `/Game/Blueprints/MilkUdders/BP_Udders` (`.ReturnValue` (`GameplayStatics.FindNearestActor` (`self.K2_GetActorLocation`) _outactors))))
  (set `self.Udders` _asbp_udders)
  (bind _outactors_2 (`GameplayStatics.GetAllActorsOfClass` "/Game/Blueprints/MilkUdders/BP_Bucket.BP_Bucket_C"))
  (bind _asbp_bucket (cast `/Game/Blueprints/MilkUdders/BP_Bucket` (`.ReturnValue` (`GameplayStatics.FindNearestActor` (`self.K2_GetActorLocation`) _outactors_2))))
  (set `self.Bucket` _asbp_bucket))

(fn `UserConstructionScript`
  (`parent.UserConstructionScript`))
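; BP_Bomb is the bomb actor in a bomb defuse game, randomizing its wire layout and exploding on a timer.
; SetLocations picks a random BP_Wire as Explode, moves each wire to an unused random left-side point and passes it a right-side point's removal before calling WireRotation.
; A 29-second timer, set inside that loop, fires Exploud, which spawns a bubble effect and gives every character's player a random score.
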(event `SetLocations`
  (bind _outactors (`GameplayStatics.GetAllActorsOfClass` "/Game/Blueprints/BombDefuse/BP_Wire.BP_Wire_C"))
  (bind _output_get (set `self.Out Actors` _outactors))
  (set `self.Explode` (`|GetArrayItem` _output_get (`KismetMathLibrary.RandomIntegerInRange` 0 (`KismetArrayLibrary.Array_LastIndex` _output_get))))
  (bind _output_get_2 (set `self.LeftSpawnLocation` (`|MakeArray` (`self.Location1`) (`self.Location3`) (`self.Location5`) (`self.Location7`))))
  (bind _output_get_3 (set `self.RightSpawnLocation` (`|MakeArray` (`self.Location2`) (`self.Location4`) (`self.Location6`) (`self.Location8`))))
  (for _array_element _output_get
    (bind _output_get_4 (set `self.FirstLocation` (`|GetArrayItem` _output_get_2 (`KismetMathLibrary.RandomIntegerInRange` 0 (`KismetArrayLibrary.Array_LastIndex` _output_get_2)))))
    (`KismetArrayLibrary.Array_RemoveItem` (`self.LeftSpawnLocation`) _output_get_4)
    (bind _output_get_5 (set `self.SecondLocation` (`|GetArrayItem` _output_get_3 (`KismetMathLibrary.RandomIntegerInRange` 0 (`KismetArrayLibrary.Array_LastIndex` _output_get_3)))))
    (`KismetArrayLibrary.Array_RemoveItem` (`self.RightSpawnLocation`) _output_get_5)
    (`self.K2_SetActorLocation` _array_element (`SceneComponent.K2_GetComponentLocation` _output_get_4) false false)
    (`/Game/Blueprints/BombDefuse/BP_Wire.WireRotation` _array_element)
    (`KismetSystemLibrary.K2_SetTimerDelegate` (delegate `Exploud`) 29.0)))

(event `Exploud`
  (`NiagaraFunctionLibrary.SpawnSystemAtLocation` "/Game/Blueprints/AmbulanceMiniGame/NS_bubble.NS_bubble" (+ (`SceneComponent.K2_GetComponentLocation` (`self.Cube`)) (0.0 -100.0 0.0)))
  (bind _outactors (`GameplayStatics.GetAllActorsOfClass` "/Game/Blueprints/BombDefuse/BP_BombDefuseCharacter.BP_BombDefuseCharacter_C"))
  (for _array_element _outactors
    (`/Game/Blueprints/FL_Functions.Add Score` (`/Game/Blueprints/BP_BasePlayer.Player` _array_element) (`KismetMathLibrary.RandomIntegerInRange` 3 10))))

(fn `UserConstructionScript`)
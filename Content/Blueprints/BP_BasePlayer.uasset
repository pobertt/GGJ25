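; BP_BasePlayer is a base player pawn that hands the view to a shared level camera and offers an example scoring event.
; On possession it caches its BP_PlayerController, gathers all BP_FloatingCamera actors and, if the first is valid, makes it the view target one tick later.
; ExampleAddScore forwards a score with the pawn's Player value to AddScore.
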(event `self.ReceivePossessed`
  (params (NewController :type "Controller Object Reference"))
  (bind _asbp_player_controller (cast `/Game/Blueprints/BP_PlayerController` NewController))
  (set `self.As BP Player Controller` _asbp_player_controller)
  (bind _outactors (`GameplayStatics.GetAllActorsOfClass` "/Game/Blueprints/BP_FloatingCamera.BP_FloatingCamera_C"))
  (bind _output_get (set `self.Cameras` _outactors))
  (bind _output (`|GetArrayItem` _output_get))
  (`/Engine/EditorBlueprintResources/StandardMacros.IsValid` _output
    (:`Is Valid`
      (`KismetSystemLibrary.DelayUntilNextTick`)
      (`PlayerController.SetViewTargetWithBlend` (`self.As BP Player Controller`) _output 0.0 "VTBlend_Linear" 0.0 false))))

(event `ExampleAddScore`
  (params (Score :type Integer))
  (`/Game/Blueprints/FL_Functions.Add Score` (`self.Player`) Score))

(fn `UserConstructionScript`)
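; Base player character for the Deep Sea Diver game, moved by input along the world Y axis only.
; On possession it caches the floating camera, adds the default Enhanced Input mapping context and tints a dynamic diver material by player slot (one of four colours).
; The move action feeds movement input, and releasing it zeroes velocity for an instant stop.
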(event `self.ReceivePossessed`
  (params (NewController :type "Controller Object Reference"))
  (`parent.ReceivePossessed` NewController)
  (bind _returnvalue (`GameplayStatics.GetActorOfClass` "/Game/Blueprints/BP_FloatingCamera.BP_FloatingCamera_C"))
  (set `self.Cam REF` _returnvalue)
  (bind _asbp_player_controller (cast `/Game/Blueprints/BP_PlayerController` NewController))
  (bind _returnvalue_2 (pcsubsystem `EnhancedInputLocalPlayerSubsystem` _asbp_player_controller))
  (`/Engine/EditorBlueprintResources/StandardMacros.IsValid` _returnvalue_2
    (:`Is Valid`
      (`EnhancedInputSubsystemInterface.AddMappingContext` _returnvalue_2 "/Game/ThirdPerson/Input/IMC_Default.IMC_Default" 0 (struct))
      (bind _returnvalue_3 (`PrimitiveComponent.CreateDynamicMaterialInstance` (`self.PlayerMesh`) 0 "/Game/Assets/DeepSeaDiver/Materials/M_Diver.M_Diver" "None"))
      (`MaterialInstanceDynamic.SetVectorParameterValue` _returnvalue_3 "Tint" (select `/Game/Blueprints/E_Player` (`self.Player`) :`NewEnumerator0` (struct :`R` 1.0 :`G` 0.018721 :`A` 1.0) :`NewEnumerator1` (struct :`R` 0.126081 :`G` 1.0 :`A` 1.0) :`NewEnumerator2` (struct :`B` 1.0 :`A` 1.0) :`NewEnumerator3` (struct :`R` 1.0 :`G` 0.883365 :`A` 1.0) :!type "LinearColor Structure")))))

(event `EnhancedInput|/Game/ThirdPerson/Input/Actions/IA_Move`
  (params (ActionValue :type "Vector2D Structure") (ElapsedSeconds :type "Float (double-precision)") (TriggeredSeconds :type "Float (double-precision)") (InputAction :type "InputAction Object Reference" :default "/Game/ThirdPerson/Input/Actions/IA_Move.IA_Move"))
  (:`Triggered`
    (`self.AddMovementInput` (0.0 1.0 0.0) ActionValue_X))
  (:`Completed`
    (set `MovementComponent.Velocity` (0.0 0.0 0.0) (`self.CharacterMovement`))))

(fn `UserConstructionScript`
  (`parent.UserConstructionScript`))
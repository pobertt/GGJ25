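; BP_Rock_DSD is a rock obstacle in the Deep Sea Diver game that knocks out players it hits.
; On hitting a diver, it enables mesh and capsule physics, applies the Ragdoll collision profile and sets the player's Hit flag.
; It then loops over all divers checking that flag, but the branch does nothing.
; A separate Hit event awards a point to its Player through a DoOnce gate.
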(event `self.Hit`
  (params (Player :type "/Game/Blueprints/E_Player Enum" :default "NewEnumerator0"))
  (`/Engine/EditorBlueprintResources/StandardMacros.DoOnce` false
    (:`Completed`
      (`/Game/Blueprints/FL_Functions.Add Score` Player 1))))

(event `self.ReceiveHit`
  (params (MyComp :type "PrimitiveComponent Object Reference") (Other :type "Actor Object Reference") (OtherComp :type "PrimitiveComponent Object Reference") (bSelfMoved :type Boolean) (HitLocation :type "Vector Structure") (HitNormal :type "Vector Structure") (NormalImpulse :type "Vector Structure") (Hit :type "HitResult Structure (by ref)"))
  (if (`KismetMathLibrary.ClassIsChildOf` (`GameplayStatics.GetObjectClass` Other) "/Game/Blueprints/BP_BasePlayer.BP_BasePlayer_C")
    (bind _asbp_base_player_dsd (cast `/Game/Blueprints/DeepSeaDiver/BP_BasePlayer_DSD` Other))
    (bind _mesh (`Character.Mesh` _asbp_base_player_dsd))
    (`PrimitiveComponent.SetSimulatePhysics` _mesh true)
    (`PrimitiveComponent.SetSimulatePhysics` (`Character.CapsuleComponent` _asbp_base_player_dsd) true)
    (`PrimitiveComponent.SetCollisionProfileName` _mesh "Ragdoll" true)
    (set `/Game/Blueprints/DeepSeaDiver/BP_BasePlayer_DSD.Hit?` true _asbp_base_player_dsd)
    (bind _outactors (`GameplayStatics.GetAllActorsOfClass` "/Game/Blueprints/DeepSeaDiver/BP_BasePlayer_DSD.BP_BasePlayer_DSD_C"))
    (for _array_element _outactors
      (if (`/Game/Blueprints/DeepSeaDiver/BP_BasePlayer_DSD.Hit?` _array_element)
        _))))

(fn `UserConstructionScript`)
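; BP_Interviewee is a one-shot interview target in the red carpet game that awards score to the player who engages it.
; GetInterviewee fires once, adding score, setting the Interviewing flag on the passed-in REF and starting a short timer.
; A timeline blends the yaw of both actors so they turn to face each other.
; When the timer fires, TalkTuah clears the flag and destroys the interviewee.
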(event `/Game/Blueprints/RedCarpet/BPI_RedCarpet.GetInterviewee`
  (params (Player :type "/Game/Blueprints/E_Player Enum" :default "NewEnumerator0") (REF :type "/Game/Blueprints/RedCarpet/BP_Interviewer Object Reference"))
  (`/Engine/EditorBlueprintResources/StandardMacros.DoOnce` false
    (:`Completed`
      (set `self.REF` REF)
      (`/Game/Blueprints/FL_Functions.Add Score` Player 2)
      (`KismetSystemLibrary.K2_SetTimerDelegate` (delegate `TalkTuah`) 2.0)
      (set `/Game/Blueprints/RedCarpet/BP_Interviewer.Interviewing` true (`self.REF`))
      (bind (_direction _newtrack_0) (`Timeline|Timeline` :!via `PlayFromStart`)
        (:`Update`
          (bind (_returnvalue_roll _returnvalue_pitch _returnvalue_yaw) (`KismetMathLibrary.BreakRotator` (`KismetMathLibrary.RLerp` (`self.K2_GetActorRotation`) (`KismetMathLibrary.FindLookAtRotation` (`self.K2_GetActorLocation`) (`self.K2_GetActorLocation` (`self.REF`))) _newtrack_0)))
          (`self.K2_SetActorRotation` (`KismetMathLibrary.MakeRotator` 0.0 0.0 _returnvalue_yaw))
          (bind (_returnvalue_roll_2 _returnvalue_pitch_2 _returnvalue_yaw_2) (`KismetMathLibrary.BreakRotator` (`KismetMathLibrary.RLerp` (`self.K2_GetActorRotation` (`self.REF`)) (`KismetMathLibrary.FindLookAtRotation` (`self.K2_GetActorLocation` (`self.REF`)) (`self.K2_GetActorLocation`)) _newtrack_0)))
          (`self.K2_SetActorRotation` (`self.REF`) (`KismetMathLibrary.MakeRotator` 0.0 0.0 _returnvalue_yaw_2) false))))))

(event `TalkTuah`
  (set `/Game/Blueprints/RedCarpet/BP_Interviewer.Interviewing` false (`self.REF`))
  (`self.K2_DestroyActor`))

(fn `UserConstructionScript`)
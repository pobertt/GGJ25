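; BP_Interviewer is a gamepad-driven player pawn that scores points by interviewing BP_Interviewee actors in a red carpet setting.
; The left stick rotates and moves it unless an interview is running.
; Box overlaps set the interviewee and open or close a gate for the right-trigger interview.
; An interview adds a point, turns both actors face to face via a timeline, then destroys the interviewee after a timer.
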(event `self.ReceivePossessed`
  (params (NewController :type "Controller Object Reference"))
  (`parent.ReceivePossessed` NewController))

(event `InputVectorAxis|Gamepad_Left2D`
  (params (AxisValue :type "Vector Structure"))
  (bind _returnvalue (`KismetMathLibrary.MakeVector` AxisValue_Y AxisValue_X))
  (bind _returnvalue_2 (`KismetMathLibrary.Normal` _returnvalue))
  (if (`KismetMathLibrary.Vector_IsNearlyZero` _returnvalue 0.1)
    _
    (elif (not (`self.Interviewing`))
      (`self.K2_SetActorRotation` (`KismetMathLibrary.Conv_VectorToRotator` _returnvalue_2))
      (`self.AddMovementInput` _returnvalue_2 (`KismetMathLibrary.VSize` _returnvalue)))))

(event `Key|Gamepad_RightTrigger`
  (params (Key :type "Key Structure"))
  (:`Pressed`
    (`self.GetInterviewee` (`self.Player`))))

(event `GetInterviewee`
  (params (Player :type "/Game/Blueprints/E_Player Enum" :default "NewEnumerator0"))
  (bind _interviewee (`self.Interviewee`))
  (`/Engine/EditorBlueprintResources/StandardMacros.Gate` true :!label _label
    (:`Exit`
      (`/Game/Blueprints/FL_Functions.Add Score` Player 1)
      (`KismetSystemLibrary.K2_SetTimerDelegate` (delegate `TalkTuah`) 2.0)
      (set `self.Interviewing` true)
      (bind (_direction _newtrack_0) (`Timeline|Timeline` :!via `PlayFromStart`)
        (:`Update`
          (bind (_returnvalue_roll _returnvalue_pitch _returnvalue_yaw) (`KismetMathLibrary.BreakRotator` (`KismetMathLibrary.RLerp` (`self.K2_GetActorRotation` _interviewee) (`KismetMathLibrary.FindLookAtRotation` (`self.K2_GetActorLocation` _interviewee) (`self.K2_GetActorLocation`)) _newtrack_0 true)))
          (`self.K2_SetActorRotation` (`self.Interviewee`) (`KismetMathLibrary.MakeRotator` 0.0 0.0 _returnvalue_yaw) false)
          (bind (_returnvalue_roll_2 _returnvalue_pitch_2 _returnvalue_yaw_2) (`KismetMathLibrary.BreakRotator` (`KismetMathLibrary.RLerp` (`self.K2_GetActorRotation`) (`KismetMathLibrary.FindLookAtRotation` (`self.K2_GetActorLocation`) (`self.K2_GetActorLocation` (`self.Interviewee`))) _newtrack_0 true)))
          (`self.K2_SetActorRotation` (`KismetMathLibrary.MakeRotator` 0.0 0.0 _returnvalue_yaw_2)))))))

(event `self.Box.OnComponentBeginOverlap`
  (params (OverlappedComponent :type "PrimitiveComponent Object Reference") (OtherActor :type "Actor Object Reference") (OtherComp :type "PrimitiveComponent Object Reference") (OtherBodyIndex :type Integer) (bFromSweep :type Boolean) (SweepResult :type "HitResult Structure (by ref)"))
  (if (== (`GameplayStatics.GetObjectClass` OtherActor) "/Game/Blueprints/RedCarpet/BP_Interviewee.BP_Interviewee_C")
    (set `self.Interviewee` OtherActor)
    (goto _label :!via `Open`)))

(event `TalkTuah`
  (bind _interviewee (`self.Interviewee`))
  (`/Engine/EditorBlueprintResources/StandardMacros.IsValid` _interviewee
    (:`Is Valid`
      (`self.K2_DestroyActor` _interviewee)
      (set `self.Interviewing` false))))

(event `self.Box.OnComponentEndOverlap`
  (params (OverlappedComponent :type "PrimitiveComponent Object Reference") (OtherActor :type "Actor Object Reference") (OtherComp :type "PrimitiveComponent Object Reference") (OtherBodyIndex :type Integer))
  (if (== (`GameplayStatics.GetObjectClass` OtherActor) "/Game/Blueprints/RedCarpet/BP_Interviewee.BP_Interviewee_C")
    (set `self.Interviewee` null)
    (goto _label :!via `Close`)))

(fn `UserConstructionScript`
  (`parent.UserConstructionScript`))
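; BP_Spatula is a player's spatula in the Teppanyaki Chef minigame, counting egg hits toward a score.
; It follows positions passed to MovetoMouse and, on the third hit, rotates its handle for a final hit.
; That next hit scores a point, then after a delay asks the owning BP_TeppanyakiTerry to spawn an egg and resets.
; On BeginPlay it takes a per-player material based on its owner's Player.
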(event `/Game/Blueprints/TeppanyakiChef/BPI_Teppanyaki.Move to Mouse`
  (params (Target :type "Vector Structure") (Player :type "/Game/Blueprints/E_Player Enum" :default "NewEnumerator0"))
  (`self.K2_SetActorLocation` Target))

(event `Egg Hit`
  (bind _result (`/Engine/EditorBlueprintResources/StandardMacros.IncrementInt` (`self.Hits`))
    (:`  `
      (if (>= _result 3)
        (if (`self.Turned?`)
          (`/Game/Blueprints/FL_Functions.Add Score` (stale `/Game/Blueprints/TeppanyakiChef/BPI_Teppanyaki.Move to Mouse` Player) 1)
          (`KismetSystemLibrary.Delay` 2.0)
          (bind _asbp_teppanyaki_terry (cast `/Game/Blueprints/TeppanyakiChef/BP_TeppanyakiTerry` (`self.GetOwner`)))
          (`/Game/Blueprints/TeppanyakiChef/BP_TeppanyakiTerry.SpawnEgg` _asbp_teppanyaki_terry)
          (`self.K2_SetActorRotation` (struct))
          (set `self.Turned?` false)
          (set `self.Hits` 0)
          (else
            ;[1 1 1] Rotates the handle for the final hit
            (`KismetSystemLibrary.Delay` 0.2)
            (`self.K2_SetActorRotation` (struct :`Roll` 90.0))
            (set `self.Turned?` true)))))))

(event `self.ReceiveBeginPlay`
  (`KismetSystemLibrary.DelayUntilNextTick`)
  (bind _asbp_teppanyaki_terry (cast `/Game/Blueprints/TeppanyakiChef/BP_TeppanyakiTerry` (`self.GetOwner`)))
  (`PrimitiveComponent.SetMaterial` (`self.Spatula_P1`) 0 (select `/Game/Blueprints/E_Player` (`/Game/Blueprints/BP_BasePlayer.Player` _asbp_teppanyaki_terry) :`NewEnumerator0` "/Game/Assets/Teppanyaki_Chef/Materials/M_Spatula_P1.M_Spatula_P1" :`NewEnumerator1` "/Game/Assets/Teppanyaki_Chef/Materials/M_Spatula_P2.M_Spatula_P2" :`NewEnumerator2` "/Game/Assets/Teppanyaki_Chef/Materials/M_Spatula_P3.M_Spatula_P3" :`NewEnumerator3` "/Game/Assets/Teppanyaki_Chef/Materials/M_Spatula_P4.M_Spatula_P4" :!type "MaterialInterface Object Reference")))

(fn `UserConstructionScript`)
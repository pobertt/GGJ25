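; BP_Egg is a physics egg for the teppanyaki chef game, juggled on a spatula until it breaks.
; Each spatula hit registers on BP_Spatula and randomly nudges and spins the egg; once the hit count reaches its limit, the egg breaks and the spatula resets.
; Hitting anything else breaks it, costs the owning Terry's player a point, respawns an egg after a delay and resets the spatula.
; Breaking swaps the sphere for a splat plane with crack and sizzle sounds.
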(event `self.Sphere.OnComponentHit`
  (params (HitComponent :type "PrimitiveComponent Object Reference") (OtherActor :type "Actor Object Reference") (OtherComp :type "PrimitiveComponent Object Reference") (NormalImpulse :type "Vector Structure") (Hit :type "HitResult Structure (by ref)"))
  (bind _asbp_spatula (cast `/Game/Blueprints/TeppanyakiChef/BP_Spatula` OtherActor)
    (:`then`
      (`/Game/Blueprints/TeppanyakiChef/BP_Spatula.Egg Hit` _asbp_spatula)
      (`self.K2_AddActorWorldRotation` (`KismetMathLibrary.MakeRotator` (`KismetMathLibrary.RandomFloatInRange` -5.0 5.0) (`KismetMathLibrary.RandomFloatInRange` -5.0 5.0) (`KismetMathLibrary.RandomFloatInRange` -5.0 5.0)))
      (`PrimitiveComponent.AddImpulse` (`self.Sphere`) (* (`KismetMathLibrary.RandomUnitVector`) (`KismetMathLibrary.RandomFloatInRange` 2.0 6.0)) "None" true)
      (if (>= (`/Game/Blueprints/TeppanyakiChef/BP_Spatula.Hits` _asbp_spatula) 4)
        (`self.Break Egg`)
        (bind _asbp_teppanyaki_terry (cast `/Game/Blueprints/TeppanyakiChef/BP_TeppanyakiTerry` (`self.GetOwner`)))
        (bind _asbp_spatula_2 (cast `/Game/Blueprints/TeppanyakiChef/BP_Spatula` (`ChildActorComponent.ChildActor` (`/Game/Blueprints/TeppanyakiChef/BP_TeppanyakiTerry.ChildActor` _asbp_teppanyaki_terry))))
        (`self.K2_SetActorRotation` :`self` _asbp_spatula_2)
        (set `/Game/Blueprints/TeppanyakiChef/BP_Spatula.Turned?` false _asbp_spatula_2)
        (set `/Game/Blueprints/TeppanyakiChef/BP_Spatula.Hits` 0 _asbp_spatula_2)))
    (:`CastFailed`
      (`self.Break Egg`)
      (bind _asbp_teppanyaki_terry_2 (cast `/Game/Blueprints/TeppanyakiChef/BP_TeppanyakiTerry` (`self.GetOwner`)))
      (`/Game/Blueprints/FL_Functions.Add Score` (`/Game/Blueprints/BP_BasePlayer.Player` _asbp_teppanyaki_terry_2) -1)
      (`KismetSystemLibrary.Delay` 2.0)
      (`/Game/Blueprints/TeppanyakiChef/BP_TeppanyakiTerry.SpawnEgg` _asbp_teppanyaki_terry_2)
      (bind _asbp_spatula_3 (cast `/Game/Blueprints/TeppanyakiChef/BP_Spatula` (`ChildActorComponent.ChildActor` (`/Game/Blueprints/TeppanyakiChef/BP_TeppanyakiTerry.ChildActor` _asbp_teppanyaki_terry_2))))
      (`self.K2_SetActorRotation` :`self` _asbp_spatula_3)
      (set `/Game/Blueprints/TeppanyakiChef/BP_Spatula.Turned?` false _asbp_spatula_3)
      (set `/Game/Blueprints/TeppanyakiChef/BP_Spatula.Hits` 0 _asbp_spatula_3))))

(event `Break Egg`
  (bind _returnvalue (`self.K2_GetActorLocation`))
  (bind (_returnvalue_x _returnvalue_y) (`KismetMathLibrary.BreakVector` (`SceneComponent.K2_GetComponentLocation` (`self.Sphere`))))
  (`SceneComponent.K2_SetWorldLocationAndRotation` :`self` (`self.Plane`) :`NewLocation` (`KismetMathLibrary.MakeVector` _returnvalue_x _returnvalue_y 101.0))
  (`ActorComponent.K2_DestroyComponent` (`self.Sphere`))
  (`SceneComponent.SetVisibility` (`self.Plane`) true false)
  (`GameplayStatics.PlaySoundAtLocation` "/Game/SoundEffects/Egg_Crack_01.Egg_Crack_01" _returnvalue (struct) 1.0 1.0 0.0 null null null null)
  (`GameplayStatics.PlaySoundAtLocation` "/Game/SoundEffects/Sizzling_01.Sizzling_01" _returnvalue (struct) 0.25 1.0 0.0 null null null null))

(fn `UserConstructionScript`)
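; BP_ChoirBoy is a clickable choir boy target in the Choir Conductor game, where players smack the current "knobhead" for points.
; BP_SpawnTheBoys is stored as its spawner along with an ID, and Identify flags the boy with a knobhead material.
; A click briefly shows the smacked material and adds or deducts score.
; A correct hit also clears the flag and calls the spawner's Reset to pick another.
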(event `Set ID`
  (params (ID :type Integer) (Spawner :type "Actor Object Reference"))
  ;[1 1 1] Stores their placement in the BP_SpawnTheBoys child actor array is locally
  (set `self.ID` ID)
  (bind _asbp_spawn_the_boys (cast `/Game/Blueprints/ChoirConductor/BP_SpawnTheBoys` Spawner))
  (set `self.Spawner` _asbp_spawn_the_boys))

(event `Identify`
  (params (`Knobhead?` :type Boolean))
  ;[1 1 1] Sets this Choir Boy as a knobhead
  (set `self.Knobhead?` true)
  (`PrimitiveComponent.SetMaterial` (`self.Plane`) 0 "/Game/Blueprints/ChoirConductor/Assets/ChoirBoys/M_CBKnobhead.M_CBKnobhead"))

(event `/Game/Blueprints/ChoirConductor/BPI_Choir.Clicked`
  (params (Player :type "/Game/Blueprints/E_Player Enum" :default "NewEnumerator0"))
  ;[1 1 1] Smacks the childs and determines whether it was deserved or not
  (`PrimitiveComponent.SetMaterial` (`self.Plane`) 0 "/Game/Blueprints/ChoirConductor/Assets/ChoirBoys/M_CBSmacked.M_CBSmacked")
  (if (`self.Knobhead?`)
    (`/Game/Blueprints/FL_Functions.Add Score` Player 1)
    (`KismetSystemLibrary.Delay` 0.2)
    ;[1 1 1] Unknobheadifies the choir boy and selects a new one
    (set `self.Knobhead?` false)
    (`/Game/Blueprints/ChoirConductor/BP_SpawnTheBoys.Reset` (`self.Spawner`))
    (else
      (`/Game/Blueprints/FL_Functions.Add Score` Player -1)
      (`KismetSystemLibrary.Delay` 0.2)))
  (`PrimitiveComponent.SetMaterial` (`self.Plane`) 0 "/Game/Blueprints/ChoirConductor/Assets/ChoirBoys/M_CBNormal.M_CBNormal"))

(fn `NormalAnimation`)

(fn `UserConstructionScript`)
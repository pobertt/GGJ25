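; Spawner for a choir conductor minigame that builds a stepped 3x5 grid of BP_ChoirBoy actors and singles one out as the "Knobhead".
; The construction script creates them as child actor components, giving each an ID, spawner reference and normal material.
; Reset, first called on BeginPlay, waits a random delay, then calls Identify on a random boy.
; SetAdjacentActors, which flags grid neighbours, is unused and kept for possible reuse.
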(event `self.ReceiveBeginPlay`
  (`self.Reset`)
  (set `self.DelayMax` 2.0))

(event `Reset`
  (bind _delaymax (`self.DelayMax`))
  (`KismetSystemLibrary.Delay` (`KismetMathLibrary.RandomFloatInRange` 0.0 (`self.DelayMax`)))
  (bind _asbp_choir_boy (cast `/Game/Blueprints/ChoirConductor/BP_ChoirBoy` (`ChildActorComponent.ChildActor` (`|GetArrayItem` (`self.ChoirBoysArray`) (`KismetMathLibrary.RandomInteger` 14)))))
  (bind _output_get (set `self.Knobhead` _asbp_choir_boy))
  (`/Game/Blueprints/ChoirConductor/BP_ChoirBoy.Identify` _output_get true)
  (if (>= 0.0 _delaymax)
    (set `self.DelayMax` (- _delaymax 0.5))))

(fn `SetAdjacentActors`
  (params (KnobheadID :type Integer))
  (locals (KnobheadNo :type Integer))
  ;[1 0 0] This function isn't needed anymore, since there won't be a "zoom" in function to investigate anymore, but I'm keeping it in case I want to reuse this minigame in a fturue project.
  ;
  ; Delete in final build of game, if you want it to be more optimised
  (set `local.KnobheadNo` KnobheadID)
  ;[1 1 1] E: Sets the child located to the right
  (bind _asbp_choir_boy (cast `/Game/Blueprints/ChoirConductor/BP_ChoirBoy` (`ChildActorComponent.ChildActor` (`|GetArrayItem` (`self.ChoirBoysArray`) (+ (`local.KnobheadNo`) 1))))
    (:`then`
      (bind _id (`/Game/Blueprints/ChoirConductor/BP_ChoirBoy.ID` _asbp_choir_boy))
      ;;[1 1 1] Ensures that the next choir boy in the array isn't on a separate row
      (if (not (or (== _id 5) (== _id 10)))
        (`/Game/Blueprints/ChoirConductor/BP_ChoirBoy.Identify` _asbp_choir_boy false)))
    (:`CastFailed`
      _))
  ;[1 1 1] W: Sets the child located to the left
  (bind _asbp_choir_boy_2 (cast `/Game/Blueprints/ChoirConductor/BP_ChoirBoy` (`ChildActorComponent.ChildActor` (`|GetArrayItem` (`self.ChoirBoysArray`) (- (`local.KnobheadNo`) 1))))
    (:`then`
      (bind _id_2 (`/Game/Blueprints/ChoirConductor/BP_ChoirBoy.ID` _asbp_choir_boy_2))
      ;;[1 1 1] Ensures that the next choir boy in the array isn't on a separate row
      (if (not (or (== _id_2 4) (== _id_2 9)))
        (`/Game/Blueprints/ChoirConductor/BP_ChoirBoy.Identify` _asbp_choir_boy_2 false)))
    (:`CastFailed`
      _))
  ;[1 1 1] S: Sets the child located below
  (bind _asbp_choir_boy_3 (cast `/Game/Blueprints/ChoirConductor/BP_ChoirBoy` (`ChildActorComponent.ChildActor` (`|GetArrayItem` (`self.ChoirBoysArray`) (- (`local.KnobheadNo`) 5))))
    (:`then`
      (`/Game/Blueprints/ChoirConductor/BP_ChoirBoy.Identify` _asbp_choir_boy_3 false))
    (:`CastFailed`
      _))
  ;[1 1 1] N: Sets the child located above
  (bind _asbp_choir_boy_4 (cast `/Game/Blueprints/ChoirConductor/BP_ChoirBoy` (`ChildActorComponent.ChildActor` (`|GetArrayItem` (`self.ChoirBoysArray`) (+ (`local.KnobheadNo`) 5))))
    (:`then`
      (`/Game/Blueprints/ChoirConductor/BP_ChoirBoy.Identify` _asbp_choir_boy_4 false))
    (:`CastFailed`
      _))
  ;[1 1 1] NE: Sets the child located above and to the right
  (bind _asbp_choir_boy_5 (cast `/Game/Blueprints/ChoirConductor/BP_ChoirBoy` (`ChildActorComponent.ChildActor` (`|GetArrayItem` (`self.ChoirBoysArray`) (+ (`local.KnobheadNo`) 6))))
    (:`then`
      (bind _id_3 (`/Game/Blueprints/ChoirConductor/BP_ChoirBoy.ID` _asbp_choir_boy_5))
      ;;[1 1 1] Ensures that the next choir boy in the array isn't on a separate row
      (if (not (or (== _id_3 5) (== _id_3 10)))
        (`/Game/Blueprints/ChoirConductor/BP_ChoirBoy.Identify` _asbp_choir_boy_5 false)))
    (:`CastFailed`
      _))
  ;[1 1 1] SW: Sets the child located below and to the left
  (bind _asbp_choir_boy_6 (cast `/Game/Blueprints/ChoirConductor/BP_ChoirBoy` (`ChildActorComponent.ChildActor` (`|GetArrayItem` (`self.ChoirBoysArray`) (- (`local.KnobheadNo`) 6))))
    (:`then`
      (bind _id_4 (`/Game/Blueprints/ChoirConductor/BP_ChoirBoy.ID` _asbp_choir_boy_6))
      ;;[1 1 1] Ensures that the next choir boy in the array isn't on a separate row
      (if (not (or (== _id_4 4) (== _id_4 9)))
        (`/Game/Blueprints/ChoirConductor/BP_ChoirBoy.Identify` _asbp_choir_boy_6 false)))
    (:`CastFailed`
      _))
  ;[1 1 1] NE: Sets the child located above and to the left
  (bind _asbp_choir_boy_7 (cast `/Game/Blueprints/ChoirConductor/BP_ChoirBoy` (`ChildActorComponent.ChildActor` (`|GetArrayItem` (`self.ChoirBoysArray`) (+ (`local.KnobheadNo`) 4))))
    (:`then`
      (bind _id_5 (`/Game/Blueprints/ChoirConductor/BP_ChoirBoy.ID` _asbp_choir_boy_7))
      ;;[1 1 1] Ensures that the next choir boy in the array isn't on a separate row
      (if (not (or (== _id_5 4) (== _id_5 9) (== _id_5 14)))
        (`/Game/Blueprints/ChoirConductor/BP_ChoirBoy.Identify` _asbp_choir_boy_7 false)))
    (:`CastFailed`
      _))
  ;[1 1 1] SE: Sets the child located below and to the right
  (bind _asbp_choir_boy_8 (cast `/Game/Blueprints/ChoirConductor/BP_ChoirBoy` (`ChildActorComponent.ChildActor` (`|GetArrayItem` (`self.ChoirBoysArray`) (- (`local.KnobheadNo`) 4)))))
  (bind _id_6 (`/Game/Blueprints/ChoirConductor/BP_ChoirBoy.ID` _asbp_choir_boy_8))
  ;;[1 1 1] Ensures that the next choir boy in the array isn't on a separate row
  (if (not (or (== _id_6 0) (== _id_6 5) (== _id_6 10)))
    (`/Game/Blueprints/ChoirConductor/BP_ChoirBoy.Identify` _asbp_choir_boy_8 false)))

(fn `UserConstructionScript`
  (for _index (range 3)
    (for _index_2 (range 5)
      (bind _returnvalue (`KismetMathLibrary.Conv_IntToDouble` (* _index 65 2)))
      (bind _returnvalue_2 (`AddComponent|NODE_AddChildActorComponent-0` :`RelativeTransform` (`KismetMathLibrary.MakeTransform` (`KismetMathLibrary.MakeVector` _returnvalue (`KismetMathLibrary.Conv_IntToDouble` (* _index_2 65 2)) _returnvalue))))
      (`KismetArrayLibrary.Array_Add` (`self.ChoirBoysArray`) _returnvalue_2)
      (`ChildActorComponent.SetChildActorClass` _returnvalue_2 "/Game/Blueprints/ChoirConductor/BP_ChoirBoy.BP_ChoirBoy_C")))
  ;[1 1 1] Stores the ID number of each of the child actors
  (for _index_3 (range 15)
    (bind _asbp_choir_boy (cast `/Game/Blueprints/ChoirConductor/BP_ChoirBoy` (`ChildActorComponent.ChildActor` (`|GetArrayItem` (`self.ChoirBoysArray`) _index_3))))
    (`/Game/Blueprints/ChoirConductor/BP_ChoirBoy.Set ID` _asbp_choir_boy _index_3 self)
    (`PrimitiveComponent.SetMaterial` (`/Game/Blueprints/ChoirConductor/BP_ChoirBoy.Plane` _asbp_choir_boy) 0 "/Game/Blueprints/ChoirConductor/Assets/ChoirBoys/M_CBNormal.M_CBNormal")))
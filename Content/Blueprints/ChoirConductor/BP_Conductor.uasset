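; BP_Conductor is the player-controlled pawn for ChoirConductor that lets the player click objects in the world.
; On possession it caches the BP_PlayerController and shows the mouse cursor.
; A left mouse press line-traces under the cursor on the Visibility channel against complex collision and sends ClickedMessage with an enum value to the hit actor.
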(event `self.ReceivePossessed`
  (params (NewController :type "Controller Object Reference"))
  (`parent.ReceivePossessed` NewController)
  (bind _asbp_player_controller (cast `/Game/Blueprints/BP_PlayerController` (`self.GetController`)))
  (set `self.As BP Player Controller` _asbp_player_controller)
  (set `PlayerController.bShowMouseCursor` true _asbp_player_controller))

(event `Key|LeftMouseButton`
  (params (Key :type "Key Structure"))
  (:`Pressed`
    (message `/Game/Blueprints/ChoirConductor/BPI_Choir.Clicked` (`.HitActor` (`GameplayStatics.BreakHitResult` (`PlayerController.GetHitResultUnderCursorByChannel` (`self.As BP Player Controller`) "TraceTypeQuery1" true))) "NewEnumerator0")))

(fn `UserConstructionScript`
  (`parent.UserConstructionScript`))